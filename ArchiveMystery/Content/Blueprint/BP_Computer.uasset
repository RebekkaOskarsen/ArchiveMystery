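; BP_Computer is an interactable computer that BP_Archivist can use to open an on-screen computer interface.
; Entering its collision volume shows the E-to-interact and dot widgets, and leaving removes them.
; InteractWith switches the view to the computer camera, disables character input and enables the mouse in UI-only mode.
; It then opens W_Computer_Screen, swaps the mesh to an email screen material and returns a "computer" identifier.
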(event `self.Collission.OnComponentBeginOverlap`
  (params (OverlappedComponent :type "PrimitiveComponent Object Reference") (OtherActor :type "Actor Object Reference") (OtherComp :type "PrimitiveComponent Object Reference") (OtherBodyIndex :type Integer) (bFromSweep :type Boolean) (SweepResult :type "HitResult Structure (by ref)"))
  ; E Widget and Dot Collission
  (cast `/Game/Blueprint/BP_Archivist` OtherActor)
  (bind _returnvalue (`|CreateWidget` "/Game/Blueprint/W_E_To_Interact.W_E_To_Interact_C"))
  (bind _output_get (set `self.Widget` _returnvalue))
  (`UserWidget.AddToViewport` _output_get 0)
  (bind _returnvalue_2 (`|CreateWidget` "/Game/Blueprint/W_Dot.W_Dot_C"))
  (bind _output_get_2 (set `self.Dot widget` _returnvalue_2))
  (`UserWidget.AddToViewport` _output_get_2 0))

(event `self.Collission.OnComponentEndOverlap`
  (params (OverlappedComponent :type "PrimitiveComponent Object Reference") (OtherActor :type "Actor Object Reference") (OtherComp :type "PrimitiveComponent Object Reference") (OtherBodyIndex :type Integer))
  ; E Widget and Dot Collission
  (cast `/Game/Blueprint/BP_Archivist` OtherActor)
  (`Widget.RemoveFromParent` (`self.Widget`))
  (`Widget.RemoveFromParent` (`self.Dot widget`)))

(fn `Interact With`
  (returns (ObjectiveID :type String))
  (bind _returnvalue (`GameplayStatics.GetPlayerController` 0))
  (`PlayerController.SetViewTargetWithBlend` (`GameplayStatics.GetPlayerController` 0) (`self.Computer Camera`) 0.0 "VTBlend_Linear" 0.0 false)
  (`/Engine/EditorBlueprintResources/StandardMacros.IsValid` _returnvalue
    (:`Is Valid`
      (`self.DisableInput` (`GameplayStatics.GetPlayerCharacter` 0) _returnvalue)
      (`WidgetBlueprintLibrary.SetInputMode_UIOnlyEx` _returnvalue null)
      (set `PlayerController.bShowMouseCursor` true _returnvalue)
      (bind _returnvalue_2 (`|CreateWidget` "/Game/Blueprint/W_Computer_Screen.W_Computer_Screen_C"))
      (`UserWidget.AddToViewport` _returnvalue_2 0)
      (`PrimitiveComponent.SetMaterial` (`self.StaticMesh`) 0 "/Game/3DAssets/Computer_And_Items/M_Computer_Screen_Email.M_Computer_Screen_Email")
      (return "computer"))))

(fn `UserConstructionScript`)