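; BP_Computer2 is a computer actor that shows a database pop-up and an outline when something overlaps its collision volume.
; Begin overlap creates a WBP_Database_PopUp, assigns it to the widget component, plays its pop-up animation and enables custom depth on the mesh for a yellow outline.
; End overlap starts the animation reversed at faster speed, but immediately hides the widget component, clears the reference and disables the outline.
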(event `self.CollisionPopUp.OnComponentBeginOverlap`
  (params (OverlappedComponent :type "PrimitiveComponent Object Reference") (OtherActor :type "Actor Object Reference") (OtherComp :type "PrimitiveComponent Object Reference") (OtherBodyIndex :type Integer) (bFromSweep :type Boolean) (SweepResult :type "HitResult Structure (by ref)"))
  (bind _widgetpopup (`self.WidgetPopUp`))
  ; CollisionBox PopUp & Outline
  (bind _returnvalue (`|CreateWidget` "/Game/Blueprint/PopUp_Widgets/WBP_Database_PopUp.WBP_Database_PopUp_C"))
  (bind _output_get (set `self.NewVar_1` _returnvalue))
  (`WidgetComponent.SetWidget` _widgetpopup _output_get)
  (`SceneComponent.SetVisibility` _widgetpopup true false)
  (bind _newvar_1 (`self.NewVar_1`)
    (:`then`
      (`UserWidget.PlayAnimation` _newvar_1 (`/Game/Blueprint/PopUp_Widgets/WBP_Database_PopUp.PopUpAnimation` _newvar_1) 0.0 1 "Forward" 1.0 false)
      ; Shows yellow outline when in box
      (`PrimitiveComponent.SetRenderCustomDepth` (`self.StaticMesh`) true))
    (:`else`)))

(event `self.CollisionPopUp.OnComponentEndOverlap`
  (params (OverlappedComponent :type "PrimitiveComponent Object Reference") (OtherActor :type "Actor Object Reference") (OtherComp :type "PrimitiveComponent Object Reference") (OtherBodyIndex :type Integer))
  ; CollisionBox PopUp & Outline
  (bind _newvar_1 (`self.NewVar_1`)
    (:`then`
      (`UserWidget.PlayAnimation` _newvar_1 (`/Game/Blueprint/PopUp_Widgets/WBP_Database_PopUp.PopUpAnimation` _newvar_1) 0.0 1 "Reverse" 2.0 false)
      (set `self.NewVar_1` null)
      (`SceneComponent.SetVisibility` (`self.WidgetPopUp`) false false)
      ; Shows yellow outline when in box
      (`PrimitiveComponent.SetRenderCustomDepth` (`self.StaticMesh`) false))
    (:`else`)))

(fn `UserConstructionScript`)