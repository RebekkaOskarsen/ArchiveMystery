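; Checkpoint trigger that saves the player's progress when a BP_Archivist overlaps its box.
; It fetches the Archivist's player save, waits behind a Delay meant to throttle repeated saves, then passes it to the game instance to save asynchronously.
; An older quest-log save to a slot remains in the graph but is disconnected and never runs.
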(event `self.Box.OnComponentBeginOverlap`
  (params (OverlappedComponent :type "PrimitiveComponent Object Reference") (OtherActor :type "Actor Object Reference") (OtherComp :type "PrimitiveComponent Object Reference") (OtherBodyIndex :type Integer) (bFromSweep :type Boolean) (SweepResult :type "HitResult Structure (by ref)"))
  (bind _asbp_archivist (cast `/Game/Blueprint/BP_Archivist` OtherActor))
  (bind _playersave (`/Game/Blueprint/BP_Archivist.GetPlayerSave` _asbp_archivist))
  ; delays so save time doesn't happen as often.
  (`KismetSystemLibrary.Delay` 5.0)
  (message `/Game/Blueprint/SaveGame/BPI_SaveGame.SavePlayer` (`GameplayStatics.GetGameInstance`) _playersave true))

(fn `UserConstructionScript`)