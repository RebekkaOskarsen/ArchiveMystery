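; Keycard-locked double door that opens when interacted with once HaveKeycard has set HasKey.
; Front and back trigger boxes track BP_Archivist, with the front showing an interact prompt or locked text by key state and the back always showing the prompt.
; The occupied box picks each leaf's swing direction, with timelines rotating the doors and reversing after a delay.
; The construction script applies the door material and locked text.
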(event `/Game/Blueprint/Lock_System/BPI_Interact.Interact`
  ; Door locked if no keycard
  (if (`self.HasKey?`)
    (`self.Open Right Door`)
    (`self.Open Left Door`)))

(event `/Game/Blueprint/Lock_System/BPI_Lock.Have Keycard`
  ; Door locked if no keycard
  (if true
    (set `self.HasKey?` true)
    (`SceneComponent.SetVisibility` (`self.TXT_Locked`) false false)
    (else
      (set `self.HasKey?` false)
      (`SceneComponent.SetVisibility` (`self.TXT_Locked`) true false))))

(event `self.Open Door Collission Front.OnComponentBeginOverlap`
  (params (OverlappedComponent :type "PrimitiveComponent Object Reference") (OtherActor :type "Actor Object Reference") (OtherComp :type "PrimitiveComponent Object Reference") (OtherBodyIndex :type Integer) (bFromSweep :type Boolean) (SweepResult :type "HitResult Structure (by ref)"))
  ; Open Collission
  (cast `/Game/Blueprint/BP_Archivist` OtherActor)
  (set `self.Player Is Inside Front Box` true)
  (if (`self.HasKey?`)
    ; Sets text visibility
    (`SceneComponent.SetVisibility` (`self.TXT_Locked`) false false)
    (bind _returnvalue (`|CreateWidget` "/Game/Blueprint/W_E_To_Interact_Long.W_E_To_Interact_Long_C"))
    (bind _output_get (set `self.Widget` _returnvalue))
    (`UserWidget.AddToViewport` _output_get 0)
    (else
      (`SceneComponent.SetVisibility` (`self.TXT_Locked`) true false))))

(event `self.Open Door Collission Front.OnComponentEndOverlap`
  (params (OverlappedComponent :type "PrimitiveComponent Object Reference") (OtherActor :type "Actor Object Reference") (OtherComp :type "PrimitiveComponent Object Reference") (OtherBodyIndex :type Integer))
  ; Open Collission
  (cast `/Game/Blueprint/BP_Archivist` OtherActor)
  (set `self.Player Is Inside Front Box` false)
  ; Sets text visibility
  (`SceneComponent.SetVisibility` (`self.TXT_Locked`) false false)
  (`Widget.RemoveFromParent` (`self.Widget`)))

(event `self.Open Door Collission Back.OnComponentBeginOverlap`
  (params (OverlappedComponent :type "PrimitiveComponent Object Reference") (OtherActor :type "Actor Object Reference") (OtherComp :type "PrimitiveComponent Object Reference") (OtherBodyIndex :type Integer) (bFromSweep :type Boolean) (SweepResult :type "HitResult Structure (by ref)"))
  ; Open Collission
  (cast `/Game/Blueprint/BP_Archivist` OtherActor)
  (set `self.Player Is Inside Back Box` true)
  (bind _returnvalue (`|CreateWidget` "/Game/Blueprint/W_E_To_Interact_Long.W_E_To_Interact_Long_C"))
  (`UserWidget.AddToViewport` _returnvalue 0))

(event `self.Open Door Collission Back.OnComponentEndOverlap`
  (params (OverlappedComponent :type "PrimitiveComponent Object Reference") (OtherActor :type "Actor Object Reference") (OtherComp :type "PrimitiveComponent Object Reference") (OtherBodyIndex :type Integer))
  ; Open Collission
  (cast `/Game/Blueprint/BP_Archivist` OtherActor)
  (set `self.Player Is Inside Back Box` false)
  (`Widget.RemoveFromParent` (stale `self.Open Door Collission Back.OnComponentBeginOverlap` _returnvalue)))

(event `Open Right Door`
  (if (`self.Player Is Inside Front Box`)
    (bind (_direction _open_door) (`Timeline|Timeline_0` :!label _label)
      (:`Update`
        (`SceneComponent.K2_SetRelativeRotation` (`self.Door_Right`) (`KismetMathLibrary.MakeRotator` 0.0 0.0 (`KismetMathLibrary.Lerp` 0.0 90.0 _open_door)) false false)
        (`KismetSystemLibrary.Delay` 7.0)
        (goto _label :!via `Reverse`)))
    (elif (`self.Player Is Inside Back Box`)
      (bind (_direction_2 _open_door_2) (`Timeline|Timeline` :!label _label_2)
        (:`Update`
          (`SceneComponent.K2_SetRelativeRotation` (`self.Door_Right`) (`KismetMathLibrary.MakeRotator` 0.0 0.0 (`KismetMathLibrary.Lerp` 0.0 -90.0 _open_door_2)) false false)
          (`KismetSystemLibrary.Delay` 7.0)
          (goto _label_2 :!via `Reverse`))))))

(event `Open Left Door`
  (if (`self.Player Is Inside Front Box`)
    (bind (_direction _open_door) (`Timeline|Timeline_1` :!label _label_3)
      (:`Update`
        (`SceneComponent.K2_SetRelativeRotation` (`self.Door_Left`) (`KismetMathLibrary.MakeRotator` 0.0 0.0 (`KismetMathLibrary.Lerp` -180.0 -270.0 _open_door)) false false)
        (`KismetSystemLibrary.Delay` 7.0)
        (goto _label_3 :!via `Reverse`)))
    (elif (`self.Player Is Inside Back Box`)
      (bind (_direction_2 _open_door_2) (`Timeline|Timeline_2` :!label _label_4)
        (:`Update`
          (`SceneComponent.K2_SetRelativeRotation` (`self.Door_Left`) (`KismetMathLibrary.MakeRotator` 0.0 0.0 (`KismetMathLibrary.Lerp` -180.0 -90.0 _open_door_2)) false false)
          (`KismetSystemLibrary.Delay` 7.0)
          (goto _label_4 :!via `Reverse`))))))

(fn `UserConstructionScript`
  (bind _material (`self.Material`))
  (`PrimitiveComponent.SetMaterial` (`self.Door_Left`) 0 _material)
  (`PrimitiveComponent.SetMaterial` (`self.Door_Right`) 0 _material)
  (`TextRenderComponent.K2_SetText` (`self.TXT_Locked`) (`self.Text on door`)))