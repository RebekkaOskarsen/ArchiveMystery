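; BP_Archivist is the player character, with interaction, right-click camera zoom, material customization and dialogue marker events.
; IA_Interact fans out to every door and URL trigger box in the level, overlapping BPI_Interact actors, and a camera trace for tagged buttons.
; It also reports LookAtActor's objective ID, but the look-at trace in InteractTrace is disconnected.
; A timeline drives zoom FOV, and BeginPlay disables ACInteractionTrace's tick when locally controlled.
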(event `self.ReceiveBeginPlay`
  ; Interaction Trace
  (`self.SetupInterActionTrace`))

(event `self.ReceiveTick`
  (params (DeltaSeconds :type "Float (single-precision)"))
  ; Interact Quest
  (`self.InteractTrace`))

(event `EnhancedInput|/Game/InputAction/IA_Archivist/IA_Interact`
  (params (ActionValue :type Boolean) (ElapsedSeconds :type "Float (double-precision)") (TriggeredSeconds :type "Float (double-precision)") (InputAction :type "InputAction Object Reference" :default "/Game/InputAction/IA_Archivist/IA_Interact.IA_Interact"))
  ; Open Door
  (:`Triggered`
    (bind _outactors (`GameplayStatics.GetAllActorsOfClass` "/Game/Blueprint/BP_Single_Door.BP_Single_Door_C"))
    (for _array_element _outactors
      (`/Game/Blueprint/BP_Single_Door.Open Door` _array_element))))

(event `EnhancedInput|/Game/InputAction/IA_Archivist/IA_Interact`
  (params (ActionValue :type Boolean) (ElapsedSeconds :type "Float (double-precision)") (TriggeredSeconds :type "Float (double-precision)") (InputAction :type "InputAction Object Reference" :default "/Game/InputAction/IA_Archivist/IA_Interact.IA_Interact"))
  ; Interact Quest
  (:`Triggered`
    (bind _look_at_actor (`self.Look At Actor`)
      (:`then`
        (bind _objectiveid (message `/Game/Blueprint/Quest_System/I_Interaction_Interface.Interact With` _look_at_actor))
        (`self.OnObjectiveIDCalled` _objectiveid))
      (:`else`))))

(event `EnhancedInput|/Game/InputAction/IA_Archivist/IA_Zoom`
  (params (ActionValue :type Boolean) (ElapsedSeconds :type "Float (double-precision)") (TriggeredSeconds :type "Float (double-precision)") (InputAction :type "InputAction Object Reference" :default "/Game/InputAction/IA_Archivist/IA_Zoom.IA_Zoom"))
  ; Right click to zoom
  (:`Started`
    (bind (_direction _zoom_track) (`Timeline|Zoom_Timeline` :!label _label)
      (:`Update`
        (`CameraComponent.SetFieldOfView` (`self.ViewCamera`) (`KismetMathLibrary.Lerp` 90.0 40.0 _zoom_track)))))
  (:`Completed`
    (goto _label :!via `Reverse`)))

(event `EnhancedInput|/Game/InputAction/IA_Archivist/IA_Interact`
  (params (ActionValue :type Boolean) (ElapsedSeconds :type "Float (double-precision)") (TriggeredSeconds :type "Float (double-precision)") (InputAction :type "InputAction Object Reference" :default "/Game/InputAction/IA_Archivist/IA_Interact.IA_Interact"))
  ; Opens Visarkiv URL if inside Triggerbox
  (:`Started`
    (bind _outactors (`GameplayStatics.GetAllActorsOfClass` "/Game/Blueprint/BP_URL_Triggerbox.BP_URL_Triggerbox_C"))
    (for _array_element _outactors
      (`/Game/Blueprint/BP_URL_Triggerbox.Open Visarkiv URL` _array_element))))

(event `EnhancedInput|/Game/InputAction/IA_Archivist/IA_Interact`
  (params (ActionValue :type Boolean) (ElapsedSeconds :type "Float (double-precision)") (TriggeredSeconds :type "Float (double-precision)") (InputAction :type "InputAction Object Reference" :default "/Game/InputAction/IA_Archivist/IA_Interact.IA_Interact"))
  ; Open Doors
  (:`Triggered`
    (bind _outactors (`GameplayStatics.GetAllActorsOfClass` "/Game/Blueprint/BP_Double_Doors.BP_Double_Doors_C"))
    (for _array_element _outactors
      (`/Game/Blueprint/BP_Double_Doors.Open Right Door` _array_element)
      (`/Game/Blueprint/BP_Double_Doors.Open Left Door` _array_element))))

(event `EnhancedInput|/Game/InputAction/IA_Archivist/IA_Interact`
  (params (ActionValue :type Boolean) (ElapsedSeconds :type "Float (double-precision)") (TriggeredSeconds :type "Float (double-precision)") (InputAction :type "InputAction Object Reference" :default "/Game/InputAction/IA_Archivist/IA_Interact.IA_Interact"))
  (bind _viewcamera (`self.ViewCamera`))
  (bind _returnvalue (`SceneComponent.K2_GetComponentLocation` _viewcamera))
  ; Line trace character - look at interaction from I Interaction Interface
  (:`Started`
    (bind (_outhit _returnvalue_2) (`KismetSystemLibrary.LineTraceSingle` _returnvalue (+ _returnvalue (* (`SceneComponent.GetForwardVector` _viewcamera) (`self.Line Trace Length`))) "TraceTypeQuery1"))
    (if _returnvalue_2
      (bind (_bblockinghit _binitialoverlap _time _distance _location _impactpoint _normal _impactnormal _physmat _hitactor _hitcomponent) (`GameplayStatics.BreakHitResult` _outhit))
      (if (`KismetSystemLibrary.DoesImplementInterface` _hitactor "/Game/Blueprint/Quest_System/I_Interaction_Interface.I_Interaction_Interface_C")
        (if (`ActorComponent.ComponentHasTag` _hitcomponent "Left Button")
          (message `/Game/Blueprint/Quest_System/I_Interaction_Interface.Look At Left` _hitactor)
          (elif (`ActorComponent.ComponentHasTag` _hitcomponent "Right Button")
            (message `/Game/Blueprint/Quest_System/I_Interaction_Interface.Look At Right` _hitactor)))))))

(event `EnhancedInput|/Game/InputAction/IA_Archivist/IA_Interact`
  (params (ActionValue :type Boolean) (ElapsedSeconds :type "Float (double-precision)") (TriggeredSeconds :type "Float (double-precision)") (InputAction :type "InputAction Object Reference" :default "/Game/InputAction/IA_Archivist/IA_Interact.IA_Interact"))
  ; Interacts
  (:`Triggered`
    (for _array_element (`self.GetOverlappingActors` "/Script/Engine.Actor")
      (if (`KismetSystemLibrary.DoesImplementInterface` _array_element "/Game/Blueprint/Lock_System/BPI_Interact.BPI_Interact_C")
        (message `/Game/Blueprint/Lock_System/BPI_Interact.Interact` _array_element)
        (break)))))

(event `Show Mold Marker`
  ; Dialogue Markers activate (will implement later)
  (`self.ShowMoldMarker`))

(event `SetCharacterMaterial`
  (params (Material :type "MaterialInterface Object Reference"))
  ; Customization Material
  (`PrimitiveComponent.SetMaterial` (`self.Mesh`) 0 Material))

(event `Show Paper Marker`
  ; Dialogue Markers activate (will implement later)
  (`self.ShowPaperMarker`))

(event `Show Missing Documents Markers`
  ; Dialogue Markers activate (will implement later)
  (`self.ShowMissingDocumentsMarker`))

(fn `GetPlayerSave`)

(fn `InteractTrace`)

(fn `SetupInterActionTrace`
  (if (`self.IsLocallyControlled`)
    (`ActorComponent.SetComponentTickEnabled` (`self.AC_InteractionTrace`) false)))

(fn `UsePlayerSave`)

(fn `UserConstructionScript`)