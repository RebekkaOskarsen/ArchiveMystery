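; BP_URL_Triggerbox is a trigger volume that lets the player open the Visarkiv website while standing inside it.
; Box overlap events for BP_Archivist set an inside flag and show or hide a text render prompt.
; The custom OpenVisarkivURL event launches the hard-coded URL only while that flag is set.
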(event `self.Box.OnComponentBeginOverlap`
  (params (OverlappedComponent :type "PrimitiveComponent Object Reference") (OtherActor :type "Actor Object Reference") (OtherComp :type "PrimitiveComponent Object Reference") (OtherBodyIndex :type Integer) (bFromSweep :type Boolean) (SweepResult :type "HitResult Structure (by ref)"))
  (cast `/Game/Blueprint/BP_Archivist` OtherActor)
  (set `self.is Character inside box?` true)
  (`SceneComponent.SetVisibility` (`self.TextRender`) true false))

(event `self.Box.OnComponentEndOverlap`
  (params (OverlappedComponent :type "PrimitiveComponent Object Reference") (OtherActor :type "Actor Object Reference") (OtherComp :type "PrimitiveComponent Object Reference") (OtherBodyIndex :type Integer))
  (cast `/Game/Blueprint/BP_Archivist` OtherActor)
  (set `self.is Character inside box?` false)
  (`SceneComponent.SetVisibility` (`self.TextRender`) false false))

(event `Open Visarkiv URL`
  (if (`self.is Character inside box?`)
    (`KismetSystemLibrary.LaunchURL` "https://www.visarkiv.no/")))

(fn `UserConstructionScript`)