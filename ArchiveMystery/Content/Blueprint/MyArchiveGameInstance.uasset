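; Game instance that keeps one-time tutorial, cutscene and customization events from replaying when the player respawns.
; DoOnce gates the cutscene, which disables player input for six seconds, and the customization event, which only stores a hitbox reference.
; Tutorial removal calls RemoveWidgetSlowly on a newly created widget, not the existing one.
; Playtutorialonce is empty, and the logic that shows the tutorial is disconnected.
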(event `Removes Tutorial Widget`
  ; Removes tutorial and cutscene and does not play again when respawn
  (bind _returnvalue (`|CreateWidget` "/Game/Blueprint/Tutorials/W_Start_Tutorial.W_Start_Tutorial_C"))
  (bind _output_get (set `self.Tutorial` _returnvalue))
  (`/Game/Blueprint/Tutorials/W_Start_Tutorial.Remove Widget Slowly` _output_get))

(event `Play tutorial once`
  ; Removes tutorial and cutscene and does not play again when respawn
)

(event `Play Cutscene once`
  (params (`start Cutscene` :type "LevelSequenceActor Object Reference"))
  (bind _returnvalue (`GameplayStatics.GetPlayerController` 0))
  (bind _returnvalue_2 (`GameplayStatics.GetPlayerCharacter` 0))
  ; Removes tutorial and cutscene and does not play again when respawn
  (`/Engine/EditorBlueprintResources/StandardMacros.DoOnce` false
    (:`Completed`
      (`MovieSceneSequencePlayer.Play` (`LevelSequenceActor.SequencePlayer` `start Cutscene`))
      (`Actor.DisableInput` _returnvalue_2 _returnvalue)
      (`KismetSystemLibrary.Delay` 6.0)
      (`Actor.EnableInput` _returnvalue_2 _returnvalue))))

(event `Play Customization Once`
  (params (`Costimization BP` :type "/Game/Blueprint/CustomizationPage/BP_Customization_Hitbox Object Reference"))
  ; Removes tutorial and cutscene and does not play again when respawn
  (`/Engine/EditorBlueprintResources/StandardMacros.DoOnce` false
    (:`Completed`
      (bind _asbp_customization_hitbox (cast `/Game/Blueprint/CustomizationPage/BP_Customization_Hitbox` `Costimization BP`))
      (set `self.Costimization BP` _asbp_customization_hitbox))))