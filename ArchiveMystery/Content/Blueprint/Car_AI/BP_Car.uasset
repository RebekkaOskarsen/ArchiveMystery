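; BP_Car is an AI car actor that drives along the spline of a BP_Path actor found in the level.
; Each Tick looks up the path with GetActorOfClass, stores it and calls StartMoving, which plays a Timeline.
; The Timeline alpha maps to distance along the spline, setting the car's world location and rotation.
; Timeline length determines speed, so there is no physics or steering.
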(event `self.ReceiveTick`
  (params (DeltaSeconds :type "Float (single-precision)"))
  (bind _returnvalue (`GameplayStatics.GetActorOfClass` "/Game/Blueprint/Car_AI/BP_Path.BP_Path_C"))
  (set `self.Path` _returnvalue)
  (`self.Start Moving`))

(event `Start Moving`
  ; Adjust timeline length for speed
  (bind (_direction _alpha) (`Timeline|Timeline`)
    (:`Update`
      (bind (_returnvalue_location _returnvalue_rotation) (`KismetMathLibrary.BreakTransform` (`SplineComponent.GetTransformAtDistanceAlongSpline` (`/Game/Blueprint/Car_AI/BP_Path.Spline` (`self.Path`)) (`KismetMathLibrary.Lerp` 0.0 (`SplineComponent.GetSplineLength` (`/Game/Blueprint/Car_AI/BP_Path.Spline` (`self.Path`))) _alpha) "World" false)))
      (`self.K2_SetActorLocationAndRotation` _returnvalue_location _returnvalue_rotation))))

(fn `UserConstructionScript`)