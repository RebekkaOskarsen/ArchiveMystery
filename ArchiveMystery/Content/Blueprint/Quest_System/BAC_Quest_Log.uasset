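; Quest log actor component that records active and completed quest IDs and answers queries about their state.
; Adding a quest spawns a BP_Quest_Base actor, kept in an array and looked up by ID.
; Completing a quest moves its ID to the completed list and fires that actor's OnQuestCompleted dispatcher.
; TrackQuest is empty, and TurnInQuest only prints a message and completes "None" instead of the passed ID.
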(fn `Add New Quest`
  (params (QuestID :type Name))
  (returns (Quest :type "/Game/Blueprint/Quest_System/BP_Quest_Base Object Reference"))
  (`KismetArrayLibrary.Array_AddUnique` (`self.Current Active Quests`) QuestID)
  (bind _returnvalue (`|SpawnActorFromClass` "/Game/Blueprint/Quest_System/BP_Quest_Base.BP_Quest_Base_C" (`KismetMathLibrary.MakeTransform` (0.0 0.0 0.0)) "Undefined" "MultiplyWithRoot" null QuestID null))
  (`KismetArrayLibrary.Array_Add` (`self.Current Quests`) _returnvalue)
  (return _returnvalue))

(fn `Complete Quest`
  (params (QuestID :type Name))
  (`KismetArrayLibrary.Array_AddUnique` (`self.Completed Quests`) QuestID)
  (`KismetArrayLibrary.Array_RemoveItem` (`self.Current Active Quests`) QuestID)
  (bind _array_element (`self.Get Quest Actor` QuestID))
  (`self.On Quest Completed` _array_element))

(fn `Get Quest Actor`
  (params (QuestID :type Name))
  (returns (`Array Element` :type "/Game/Blueprint/Quest_System/BP_Quest_Base Object Reference"))
  (for _array_element (`self.Current Quests`)
    (if (== (`/Game/Blueprint/Quest_System/BP_Quest_Base.QuestID` _array_element) QuestID)
      (return _array_element))))

(fn `Query Active Quest`
  (params (QuestID :type Name))
  (returns (ReturnValue :type Boolean))
  (return (`KismetArrayLibrary.Array_Contains` (`self.Current Active Quests`) QuestID)))

(fn `Query Completed Quest`
  (params (QuestID :type Name))
  (returns (ReturnValue :type Boolean) (`Turned In` :type Boolean))
  (bind _returnvalue (`KismetArrayLibrary.Array_Contains` (`self.Completed Quests`) QuestID))
  (bind _array_element (`self.Get Quest Actor` QuestID))
  (`/Engine/EditorBlueprintResources/StandardMacros.IsValid` _array_element
    (:`Is Valid`
      (return _returnvalue (`/Game/Blueprint/Quest_System/BP_Quest_Base.Is Turned In` _array_element)))
    (:`Is Not Valid`
      (return _returnvalue true))))

(fn `Track Quest`)

(fn `Turn In Quest`
  (params (QuestID :type Name))
  (`|ExecutionSequence`
    (:`then_0`
      (bind _array_element (`self.Get Quest Actor` QuestID))
      (`KismetSystemLibrary.PrintString` (`KismetTextLibrary.Conv_TextToString` (`|FormatText` "Quest Finished"))))
    (:`then_1`
      (`self.Complete Quest` "None"))))