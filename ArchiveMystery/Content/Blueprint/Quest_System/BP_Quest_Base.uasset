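; Base quest actor that tracks a player's progress through one staged quest.
; It loads stages and objectives from DT_Quest_Data by QuestID and keeps per-objective counts in a map.
; Objective ID events from the player character increment counts up to their required quantities and raise an update notification.
; Finishing all objectives advances the stage; after the last, it marks completion and optionally auto-turns in through the quest log component.
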(event `self.ReceiveBeginPlay`
  (`self.Get Quest Details`)
  (add `/Game/Blueprint/BP_Archivist.OnObjectiveIDCalled` (`/Game/Blueprint/Quest_System/BFL_Common_Function_Library.Get My Player Character`) (`|CreateDelegate` :!event `On Objective ID Heard`))
  (for _ (`.Stages_18_8E14AB6841B4A8BE590A5798B28D3AA0` (break `/Game/Blueprint/Quest_System/S_Quest_Details` (`self.Quest Details`)))
    _)
  (`KismetSystemLibrary.Delay` 1.0)
  (bind _return (`self.Are Objectives Complete`))
  (set `self.Is Completed` _return))

(fn `Are Objectives Complete`
  (returns (Return :type Boolean))
  (locals (Local_All_Complete :type Boolean :default true))
  (for _array_element (`.Objectives_10_20491B6442248EB152F2DE8E584F0331` (break `/Game/Blueprint/Quest_System/S_Stage_Details` (`self.Current Stage Details`)))
    (bind (_objectivename _description _type _objectiveid) (break `/Game/Blueprint/Quest_System/S_Objective_Details` _array_element))
    (if (not (>= (`BlueprintMapLibrary.Map_Find` (`self.Current Objective Progress`) _objectiveid) (`.Quantity_15_B28B7BDB4B2DA5C3C1011EB92F707C3C` (break `/Game/Blueprint/Quest_System/S_Objective_Details` (`self.Get Objective Data By ID` _objectiveid)))))
      (bind _output_get (set `local.Local_All_Complete` false))
      (return _output_get)))
  (return (`local.Local_All_Complete`)))

(fn `Get Objective Data By ID`
  (params (ObjectiveID :type String))
  (returns (`Array Element` :type "/Game/Blueprint/Quest_System/S_Objective_Details Structure"))
  (for _array_element (`.Objectives_10_20491B6442248EB152F2DE8E584F0331` (break `/Game/Blueprint/Quest_System/S_Stage_Details` (`self.Current Stage Details`)))
    (if (`KismetStringLibrary.EqualEqual_StrStr` (`.ObjectiveID_17_0AE70EFE4DDBB25E60684FAA5D45F296` (break `/Game/Blueprint/Quest_System/S_Objective_Details` _array_element)) ObjectiveID)
      (return _array_element))))

(fn `Get Quest Details`
  (bind _returnvalue (`|GetDataTableRow` "/Game/Blueprint/Quest_System/DT_Quest_Data.DT_Quest_Data" (`self.QuestID`))
    (:`then`
      (bind _output_get (set `self.Quest Details` _returnvalue))
      (bind _output_get_2 (set `self.Current Stage Details` (`|GetArrayItem` (`.Stages_18_8E14AB6841B4A8BE590A5798B28D3AA0` (break `/Game/Blueprint/Quest_System/S_Quest_Details` _output_get)) (`self.Current Stage`))))
      (`BlueprintMapLibrary.Map_Clear` (`self.Current Objective Progress`))
      (for _array_element (`.Objectives_10_20491B6442248EB152F2DE8E584F0331` (break `/Game/Blueprint/Quest_System/S_Stage_Details` _output_get_2))
        (`BlueprintMapLibrary.Map_Add` (`self.Current Objective Progress`) (`.ObjectiveID_17_0AE70EFE4DDBB25E60684FAA5D45F296` (break `/Game/Blueprint/Quest_System/S_Objective_Details` _array_element)))))))

(fn `Is Objective Complete`
  (params (ObjectiveID :type String))
  (bind (_quest_details_name _quest_details_description _quest_details_trackingdescription _quest_details_ismainquest _quest_details_stages) (break `/Game/Blueprint/Quest_System/S_Quest_Details` (`self.Quest Details`)))
  (bind (_quest_details_name_2 _quest_details_description_2 _quest_details_trackingdescription_2 _quest_details_ismainquest_2 _quest_details_stages_2 _quest_details_autoaccept _quest_details_autocomplete) (break `/Game/Blueprint/Quest_System/S_Quest_Details` (`self.Quest Details`)))
  (if (>= (`BlueprintMapLibrary.Map_Find` (`self.Current Objective Progress`) (`local.ObjectiveID`)) (`.Quantity_15_B28B7BDB4B2DA5C3C1011EB92F707C3C` (break `/Game/Blueprint/Quest_System/S_Objective_Details` (`self.Get Objective Data By ID` ObjectiveID))))
    (bind _return (`self.Are Objectives Complete`))
    (if _return
      (bind _result (`/Engine/EditorBlueprintResources/StandardMacros.IncrementInt` (`self.Current Stage`))
        (:`  `
          (if (`KismetArrayLibrary.Array_IsValidIndex` _quest_details_stages _result)
            (`self.Get Quest Details`)
            (else
              (set `self.Is Completed` true)
              (if _quest_details_autocomplete
                (`/Game/Blueprint/Quest_System/BAC_Quest_Log.Turn In Quest` (`self.GetComponentByClass` (`GameplayStatics.GetPlayerCharacter` 0) "/Game/Blueprint/Quest_System/BAC_Quest_Log.BAC_Quest_Log_C") (`self.QuestID`))))))))))

(fn `On Objective ID Heard`
  (params (ObjectiveID :type String))
  (bind _objectiveid (`local.ObjectiveID`))
  (bind (_value _returnvalue) (`BlueprintMapLibrary.Map_Find` (`self.Current Objective Progress`) ObjectiveID))
  (if _returnvalue
    (if (< _value (`.Quantity_15_B28B7BDB4B2DA5C3C1011EB92F707C3C` (break `/Game/Blueprint/Quest_System/S_Objective_Details` (`self.Get Objective Data By ID` ObjectiveID))))
      (`BlueprintMapLibrary.Map_Add` (`self.Current Objective Progress`) _objectiveid (+ _value 1))
      (`self.Is Objective Complete` _objectiveid)
      (`self.OnObjectiveHeard`)
      (return))
    (else
      (return))))

(fn `UpdateQuestDetails`
  (bind _returnvalue (`|GetDataTableRow` "/Game/Blueprint/Quest_System/DT_Quest_Data.DT_Quest_Data" (`self.QuestID`))
    (:`then`
      (bind _output_get (set `self.Quest Details` _returnvalue))
      (set `self.Current Stage Details` (`|GetArrayItem` (`.Stages_18_8E14AB6841B4A8BE590A5798B28D3AA0` (break `/Game/Blueprint/Quest_System/S_Quest_Details` _output_get)) (`self.Current Stage`))))))

(fn `UserConstructionScript`)