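; BP_QuestGiver is a Blueprint that hands a configured quest to the player.
; On BeginPlay it calls GiveQuest, so the quest is granted automatically with no interaction.
; GiveQuest passes the QuestData row name to the player character's BACQuestLog component, adding the quest only if QueryActiveQuest reports it is not already active.
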(event `self.ReceiveBeginPlay`
  (`self.Give Quest`))

(event `Give Quest`
  (bind (_questdata_datatable _questdata_rowname) (break `DataTableRowHandle` (`self.QuestData`)))
  (bind (_questdata_datatable_2 _questdata_rowname_2) (break `DataTableRowHandle` (`self.QuestData`)))
  (if (not (`/Game/Blueprint/Quest_System/BAC_Quest_Log.Query Active Quest` (`/Game/Blueprint/BP_Archivist.BAC_Quest_Log` (`/Game/Blueprint/Quest_System/BFL_Common_Function_Library.Get My Player Character`)) _questdata_rowname))
    (`/Game/Blueprint/Quest_System/BAC_Quest_Log.Add New Quest` (`/Game/Blueprint/BP_Archivist.BAC_Quest_Log` (`/Game/Blueprint/Quest_System/BFL_Common_Function_Library.Get My Player Character`)) _questdata_rowname_2)))

(fn `UserConstructionScript`)