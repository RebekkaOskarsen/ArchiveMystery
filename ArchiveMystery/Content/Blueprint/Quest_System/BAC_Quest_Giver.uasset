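; Quest giver actor component that offers a data table quest to the player and presents its rewards on completion.
; InteractWith checks the player's quest log, then either auto-accepts a new quest or opens the delivery organization widget with its details.
; For quests already logged, it shows the rewards widget if the quest actor is completed but not turned in.
; Handled interactions return the owner's display name.
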(fn `Display Quest`
  (bind (_quest_data_datatable _quest_data_rowname) (break `DataTableRowHandle` (`self.Quest Data`)))
  (bind _returnvalue (`|GetDataTableRow` _quest_data_datatable _quest_data_rowname)
    (:`then`
      (bind _returnvalue_2 (`|CreateWidget` "/Game/Blueprint/Quest_System/UI/W_Delivery_Organization.W_Delivery_Organization_C" null _returnvalue _quest_data_rowname))
      (`UserWidget.AddToViewport` _returnvalue_2 0))))

(fn `DisplayRewards`
  (bind (_quest_data_datatable _quest_data_rowname) (break `DataTableRowHandle` (`self.Quest Data`)))
  (bind _returnvalue (`|GetDataTableRow` "/Game/Blueprint/Quest_System/DT_Quest_Data.DT_Quest_Data" _quest_data_rowname)
    (:`then`
      (bind _returnvalue_2 (`|CreateWidget` "/Game/Blueprint/Quest_System/UI/W_Delivery_Rewards.W_Delivery_Rewards_C" null _returnvalue _quest_data_rowname))
      (`UserWidget.AddToViewport` _returnvalue_2 0))))

(fn `Interact With`
  (returns (ObjectiveID :type String))
  (bind (_quest_data_datatable _quest_data_rowname) (break `DataTableRowHandle` (`self.Quest Data`)))
  (bind (_quest_data_datatable_2 _quest_data_rowname_2) (break `DataTableRowHandle` (`self.Quest Data`)))
  (bind (_quest_data_datatable_3 _quest_data_rowname_3) (break `DataTableRowHandle` (`self.Quest Data`)))
  (bind (_quest_data_datatable_4 _quest_data_rowname_4) (break `DataTableRowHandle` (`self.Quest Data`)))
  (bind _returnvalue (`Actor.GetComponentByClass` (`GameplayStatics.GetPlayerCharacter` 0) "/Game/Blueprint/Quest_System/BAC_Quest_Log.BAC_Quest_Log_C"))
  (bind _returnvalue_2 (`KismetSystemLibrary.GetDisplayName` (`self.GetOwner`)))
  (bind _bac_quest_log (`/Game/Blueprint/BP_Archivist.BAC_Quest_Log` (`/Game/Blueprint/Quest_System/BFL_Common_Function_Library.Get My Player Character`)))
  (if (and (not (`/Game/Blueprint/Quest_System/BAC_Quest_Log.Query Active Quest` _bac_quest_log _quest_data_rowname_2)) (not (`/Game/Blueprint/Quest_System/BAC_Quest_Log.Query Completed Quest` _bac_quest_log _quest_data_rowname_2)))
    (bind _returnvalue_3 (`|GetDataTableRow` "/Game/Blueprint/Quest_System/DT_Quest_Data.DT_Quest_Data" _quest_data_rowname_4)
      (:`then`
        (if (`.AutoAccept_21_28732B7043609C7C22CD80B7E003FFD2` (break `/Game/Blueprint/Quest_System/S_Quest_Details` _returnvalue_3))
          (`/Engine/EditorBlueprintResources/StandardMacros.IsValid` _returnvalue
            (:`Is Valid`
              (`/Game/Blueprint/Quest_System/BAC_Quest_Log.Add New Quest` _returnvalue _quest_data_rowname_3)
              (return (`KismetSystemLibrary.GetDisplayName` (`self.GetOwner`)))))
          (else
            (`self.Display Quest`)
            (return _returnvalue_2)))))
    (else
      (bind _array_element (`/Game/Blueprint/Quest_System/BAC_Quest_Log.Get Quest Actor` (`/Game/Blueprint/BP_Archivist.BAC_Quest_Log` (`/Game/Blueprint/Quest_System/BFL_Common_Function_Library.Get My Player Character`)) _quest_data_rowname))
      (if (and (`/Game/Blueprint/Quest_System/BP_Quest_Base.Is Completed` _array_element) (not (`/Game/Blueprint/Quest_System/BP_Quest_Base.Is Turned In` _array_element)))
        (`self.DisplayRewards`)
        (return _returnvalue_2)))))