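; Quest checkpoint tracker that numbers an ordered list of checkpoints and handles their cleared notifications for a course.
; StartSequence numbers each checkpoint, binds its cleared callback and plays level music, all inside loops, while requesting activation of the first.
; CheckpointCleared calls LapCheck, which ignores its input and always targets the first checkpoint.
; ActivateCheckpoint and ApplySettings are empty, with the trigger, Niagara and widget activation nodes left unconnected.
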(event `self.ReceiveBeginPlay`
  (bind _asmy_player_controller (cast `/Game/FirstPerson/Blueprints/My_Player_Controller` (`GameplayStatics.GetPlayerController` 0)))
  (set `self.Controller Reference` _asmy_player_controller)
  (`self.Apply Settings`))

(event `Apply Settings`)

(event `Start Sequence`
  (bind _checkpoints (`self.Checkpoints`))
  ; Start Sequence, activates checkpoints
  (for (_array_element _array_index) (`self.Checkpoints`)
    (set `/Game/Blueprint/Quest_System/BP_Checkpoint.CheckpointNumber` (+ _array_index 1) _array_element)
    (set `self.Total Checkpoints` (`KismetArrayLibrary.Array_Length` _checkpoints))
    (`self.Activate Checkpoint` (`|GetArrayItem` _checkpoints))
    (for _array_element_2 (`self.Checkpoints`)
      (add `/Game/Blueprint/Quest_System/BP_Checkpoint.Checkpoint Cleared` _array_element_2 (delegate `Checkpoint Cleared`))
      (`AudioComponent.Play` (`AmbientSound.AudioComponent` (`self.Level Music`)) 0.0))))

(event `Checkpoint Cleared`
  (params (NextCheckpoint :type Integer))
  ; Start Sequence, activates checkpoints
  (`self.Lap Check` 0))

(fn `Activate Checkpoint`
  (params (NextCheckpoint :type "/Game/Blueprint/Quest_System/BP_Checkpoint Object Reference"))
  ; Activates next checkpoint
)

(fn `Lap Check`
  (params (Checkpoint :type Integer))
  (locals (`Local Checkpoint` :type Integer))
  (bind _output_get (set `local.Local Checkpoint` 0))
  (if (not (== _output_get (`self.Total Checkpoints`)))
    (`self.Activate Checkpoint` (`|GetArrayItem` (`self.Checkpoints`) (`local.Local Checkpoint`)))))

(fn `UserConstructionScript`)