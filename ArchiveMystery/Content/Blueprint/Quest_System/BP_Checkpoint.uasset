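; A quest checkpoint actor that registers when the player character, BP_Archivist, passes through it in the intended direction.
; On BeginPlay it gives its quest marker widget the actor's location as origin.
; When the Archivist leaves the trigger moving along the Arrow's forward vector, checked by a velocity dot product, it fires the CheckpointCleared dispatcher with its number.
; It then hides the trigger, Niagara effect and widget and disables further overlaps.
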(event `self.ReceiveBeginPlay`
  (bind _asw_quest_marker (cast `/Game/Blueprint/Quest_System/UI/W_Quest_Marker` (`WidgetComponent.GetWidget` (`self.Widget`))))
  (set `/Game/Blueprint/Quest_System/UI/W_Quest_Marker.OriginLocation` (`self.K2_GetActorLocation`) _asw_quest_marker))

(event `self.Trigger.OnComponentEndOverlap`
  (params (OverlappedComponent :type "PrimitiveComponent Object Reference") (OtherActor :type "Actor Object Reference") (OtherComp :type "PrimitiveComponent Object Reference") (OtherBodyIndex :type Integer))
  (bind _trigger (`self.Trigger`))
  ; Checkpoint System
  (bind _asbp_archivist (cast `/Game/Blueprint/BP_Archivist` OtherActor))
  (if (> (`KismetMathLibrary.Dot_VectorVector` (`self.GetVelocity` _asbp_archivist) (`KismetMathLibrary.Conv_RotatorToVector` (`SceneComponent.K2_GetComponentRotation` (`self.Arrow`)))) 0.0)
    (`self.Checkpoint Cleared` (`self.CheckpointNumber`))
    (`SceneComponent.SetHiddenInGame` _trigger true false)
    (`SceneComponent.SetHiddenInGame` (`self.Niagara`) true false)
    (`SceneComponent.SetHiddenInGame` (`self.Widget`) true false)
    (set `PrimitiveComponent.bGenerateOverlapEvents` false _trigger)
    (`SceneComponent.SetVisibility` (`self.Widget`) true false)
    (`SceneComponent.SetVisibility` (`self.Trigger`) true false)))

(fn `UserConstructionScript`)