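; Archive ghost NPC that gives the archivist help on quests, the paper and mold minigames, the database, and exploration.
; Capsule overlap with BP_Archivist toggles an interact prompt, while Interact opens the WBP_Dialogue widget created at BeginPlay.
; ContinueDialogue switches on the widget's GhostTimesSpoken to set ghost lines, option texts and button states, or close the dialogue.
; Some branches rewrite that counter to redirect the conversation flow.
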(event `self.ReceiveBeginPlay`
  ; Create REF to dialogue widget
  (bind _returnvalue (`|CreateWidget` "/Game/Dialogue/WBP_Dialogue.WBP_Dialogue_C"))
  (set `self.Dialogue_Widget_REF` _returnvalue))

(event `Hide Interact`
  ; Interact Widget
  (if (`self.Is_Dialogue_Open?`) :!label _label
    (`Widget.RemoveFromParent` (stale `self.Capsule Collision.OnComponentEndOverlap` _w_interact) :!label _label_2)
    (else
      (cast `/Game/Blueprint/BP_Archivist` (stale `self.Capsule Collision.OnComponentBeginOverlap` OtherActor))
      (bind _returnvalue (`|CreateWidget` "/Game/Blueprint/W_E_To_Interact.W_E_To_Interact_C"))
      (bind _output_get (set `self.W_Interact` _returnvalue))
      (`UserWidget.AddToViewport` _output_get 0))))

(event `self.Capsule Collision.OnComponentBeginOverlap`
  (params (OverlappedComponent :type "PrimitiveComponent Object Reference") (OtherActor :type "Actor Object Reference") (OtherComp :type "PrimitiveComponent Object Reference") (OtherBodyIndex :type Integer) (bFromSweep :type Boolean) (SweepResult :type "HitResult Structure (by ref)"))
  ; Interact Widget
  (goto _label))

(event `self.Capsule Collision.OnComponentEndOverlap`
  (params (OverlappedComponent :type "PrimitiveComponent Object Reference") (OtherActor :type "Actor Object Reference") (OtherComp :type "PrimitiveComponent Object Reference") (OtherBodyIndex :type Integer))
  ; Interact Widget
  (cast `/Game/Blueprint/BP_Archivist` OtherActor)
  (bind _w_interact (`self.W_Interact`)
    (:`then`
      (goto _label_2))
    (:`else`)))

(event `/Game/Blueprint/Lock_System/BPI_Interact.Continue Dialogue`
  (bind _dialogue_widget_ref (`self.Dialogue_Widget_REF`))
  (bind _dialogue_widget_ref_2 (`self.Dialogue_Widget_REF`))
  (bind _dialogue_widget_ref_3 (`self.Dialogue_Widget_REF`))
  (bind _dialogue_widget_ref_4 (`self.Dialogue_Widget_REF`))
  (bind _dialogue_widget_ref_5 (`self.Dialogue_Widget_REF`))
  (bind _dialogue_widget_ref_6 (`self.Dialogue_Widget_REF`))
  (bind _dialogue_widget_ref_7 (`self.Dialogue_Widget_REF`))
  (bind _dialogue_widget_ref_8 (`self.Dialogue_Widget_REF`))
  (bind _dialogue_widget_ref_9 (`self.Dialogue_Widget_REF`))
  (bind _dialogue_widget_ref_10 (`self.Dialogue_Widget_REF`))
  (bind _dialogue_widget_ref_11 (`self.Dialogue_Widget_REF`))
  (bind _dialogue_widget_ref_12 (`self.Dialogue_Widget_REF`))
  (bind _dialogue_widget_ref_13 (`self.Dialogue_Widget_REF`))
  (bind _dialogue_widget_ref_14 (`self.Dialogue_Widget_REF`))
  (bind _dialogue_widget_ref_15 (`self.Dialogue_Widget_REF`))
  (bind _dialogue_widget_ref_16 (`self.Dialogue_Widget_REF`))
  ; When Interacted with add the dialogue widget to the viewport, hide the interact widget, and choose dialogue based on Ghost Times Spoken number
  (switch `int` (`/Game/Dialogue/WBP_Dialogue.Ghost_Times_Spoken` (`self.Dialogue_Widget_REF`)) :!label _label_3
    (:`1`
      ; Ghost Times Spoken: 1
      (`Widget.SetVisibility` (`/Game/Dialogue/WBP_Dialogue.Player_Dialogue_Box` _dialogue_widget_ref_13) "Visible")
      (`Widget.SetVisibility` (`/Game/Dialogue/WBP_Dialogue.Continue_Button` _dialogue_widget_ref_13) "Hidden")
      (set `/Game/Dialogue/WBP_Dialogue.Ghost_Text` "Hello archivist, need something?" _dialogue_widget_ref_13)
      (set `/Game/Dialogue/WBP_Dialogue.Option1_Text` "I need help..." _dialogue_widget_ref_13)
      (set `/Game/Dialogue/WBP_Dialogue.Option2_Text` "Who are you?" _dialogue_widget_ref_13)
      (set `/Game/Dialogue/WBP_Dialogue.Option3_Text` "About the archive..." _dialogue_widget_ref_13)
      (`Widget.SetIsEnabled` (`/Game/Dialogue/WBP_Dialogue.Option_3_Button` _dialogue_widget_ref_13) true)
      (set `/Game/Dialogue/WBP_Dialogue.Option4_Text` "I'm good" _dialogue_widget_ref_13)
      (`Widget.SetIsEnabled` (`/Game/Dialogue/WBP_Dialogue.Option_4_Button` _dialogue_widget_ref_13) true))
    (:`2`
      ; Ghost Times Spoken: 2
      (set `/Game/Dialogue/WBP_Dialogue.Ghost_Text` "What do you need help with?" _dialogue_widget_ref)
      (set `/Game/Dialogue/WBP_Dialogue.Option1_Text` "Anything..." _dialogue_widget_ref)
      (set `/Game/Dialogue/WBP_Dialogue.Option2_Text` "Paper Game..." _dialogue_widget_ref)
      (set `/Game/Dialogue/WBP_Dialogue.Option3_Text` "Mold Game..." _dialogue_widget_ref)
      (`Widget.SetIsEnabled` (`/Game/Dialogue/WBP_Dialogue.Option_3_Button` _dialogue_widget_ref) true)
      (set `/Game/Dialogue/WBP_Dialogue.Option4_Text` "Database..." _dialogue_widget_ref)
      (`Widget.SetIsEnabled` (`/Game/Dialogue/WBP_Dialogue.Option_4_Button` _dialogue_widget_ref) true)
      (`Widget.SetVisibility` (`/Game/Dialogue/WBP_Dialogue.Continue_Button` _dialogue_widget_ref) "Hidden"))
    (:`3`
      ; Ghost Times Spoken: 3
      (set `/Game/Dialogue/WBP_Dialogue.Ghost_Text` "Make sure to follow the Yellow Quest Markers." _dialogue_widget_ref_5)
      (`Widget.SetVisibility` (`/Game/Dialogue/WBP_Dialogue.Continue_Button` _dialogue_widget_ref_5) "Visible")
      (`Widget.SetVisibility` (`/Game/Dialogue/WBP_Dialogue.Player_Dialogue_Box` _dialogue_widget_ref_5) "Hidden"))
    (:`4`
      ; Ghost Times Spoken: 4
      (set `/Game/Dialogue/WBP_Dialogue.Ghost_Text` "If you are stuck; check your Quest Log by pressing TAB. All your tasks are noted there in detail." _dialogue_widget_ref_6)
      (`Widget.SetVisibility` (`/Game/Dialogue/WBP_Dialogue.Continue_Button` _dialogue_widget_ref_6) "Visible")
      (`Widget.SetVisibility` (`/Game/Dialogue/WBP_Dialogue.Player_Dialogue_Box` _dialogue_widget_ref_6) "Hidden"))
    (:`5`
      ; Ghost Times Spoken: 5
      (set `/Game/Dialogue/WBP_Dialogue.Ghost_Text` "Do walk around a bit, there's many things to interact with and see." _dialogue_widget_ref_8)
      (`Widget.SetVisibility` (`/Game/Dialogue/WBP_Dialogue.Continue_Button` _dialogue_widget_ref_8) "Visible")
      (`Widget.SetVisibility` (`/Game/Dialogue/WBP_Dialogue.Player_Dialogue_Box` _dialogue_widget_ref_8) "Hidden")
      (set `/Game/Dialogue/WBP_Dialogue.Ghost_Times_Spoken` 0 _dialogue_widget_ref_8))
    (:`6`
      ; Ghost Times Spoken: 6
      (set `/Game/Dialogue/WBP_Dialogue.Ghost_Text` "To find the shredded paper minigame, go to the Office and to the long tables to the left. A glovebox should light up if you go close." _dialogue_widget_ref_9)
      (`Widget.SetVisibility` (`/Game/Dialogue/WBP_Dialogue.Continue_Button` _dialogue_widget_ref_9) "Visible")
      (`Widget.SetVisibility` (`/Game/Dialogue/WBP_Dialogue.Player_Dialogue_Box` _dialogue_widget_ref_9) "Hidden"))
    (:`7`
      ; Ghost Times Spoken: 7
      (set `/Game/Dialogue/WBP_Dialogue.Ghost_Text` "Anything else you wonder?" _dialogue_widget_ref_7)
      (`Widget.SetVisibility` (`/Game/Dialogue/WBP_Dialogue.Player_Dialogue_Box` _dialogue_widget_ref_7) "Visible")
      (`Widget.SetVisibility` (`/Game/Dialogue/WBP_Dialogue.Continue_Button` _dialogue_widget_ref_7) "Hidden")
      (set `/Game/Dialogue/WBP_Dialogue.Option1_Text` "No thanks" _dialogue_widget_ref_7)
      (set `/Game/Dialogue/WBP_Dialogue.Option2_Text` "Yes please" _dialogue_widget_ref_7)
      (set `/Game/Dialogue/WBP_Dialogue.Option3_Text` "" _dialogue_widget_ref_3)
      (`Widget.SetIsEnabled` (`/Game/Dialogue/WBP_Dialogue.Option_3_Button` _dialogue_widget_ref_3) false)
      (set `/Game/Dialogue/WBP_Dialogue.Option4_Text` "" _dialogue_widget_ref_3)
      (`Widget.SetIsEnabled` (`/Game/Dialogue/WBP_Dialogue.Option_4_Button` _dialogue_widget_ref_3) false))
    (:`8`
      ; Ghost Times Spoken: 8
      (set `/Game/Dialogue/WBP_Dialogue.Ghost_Text` "Go to the Mold Clearance Room in the Office and check the fume hood. If it doesn't work, then you need to finish the shredded paper minigame first." _dialogue_widget_ref_11)
      (`Widget.SetVisibility` (`/Game/Dialogue/WBP_Dialogue.Continue_Button` _dialogue_widget_ref_11) "Visible")
      (`Widget.SetVisibility` (`/Game/Dialogue/WBP_Dialogue.Player_Dialogue_Box` _dialogue_widget_ref_11) "Hidden")
      (set `/Game/Dialogue/WBP_Dialogue.Ghost_Times_Spoken` 6 _dialogue_widget_ref_11))
    (:`9`
      ; Ghost Times Spoken: 9
      (set `/Game/Dialogue/WBP_Dialogue.Ghost_Text` "Database (SQL) is a digital system where information the archive receives is sorted into categories and stored for later use." _dialogue_widget_ref_4)
      (`Widget.SetVisibility` (`/Game/Dialogue/WBP_Dialogue.Player_Dialogue_Box` _dialogue_widget_ref_4) "Visible")
      (`Widget.SetVisibility` (`/Game/Dialogue/WBP_Dialogue.Continue_Button` _dialogue_widget_ref_4) "Hidden"))
    (:`10`
      ; Ghost Times Spoken: 10
      (set `/Game/Dialogue/WBP_Dialogue.Ghost_Text` "Database is kind of complicated to understand, but reading the guide shown as a book icon on the computer can help you figure out what to search for." _dialogue_widget_ref_12)
      (`Widget.SetVisibility` (`/Game/Dialogue/WBP_Dialogue.Continue_Button` _dialogue_widget_ref_12) "Visible")
      (`Widget.SetVisibility` (`/Game/Dialogue/WBP_Dialogue.Player_Dialogue_Box` _dialogue_widget_ref_12) "Hidden"))
    (:`11`
      ; Ghost Times Spoken: 11
      (set `/Game/Dialogue/WBP_Dialogue.Ghost_Text` "There are left hints inside the guide, read them carefully and you will be able to find out where the information lies." _dialogue_widget_ref_10)
      (`Widget.SetVisibility` (`/Game/Dialogue/WBP_Dialogue.Player_Dialogue_Box` _dialogue_widget_ref_10) "Hidden")
      (`Widget.SetVisibility` (`/Game/Dialogue/WBP_Dialogue.Continue_Button` _dialogue_widget_ref_10) "Visible")
      (set `/Game/Dialogue/WBP_Dialogue.Ghost_Times_Spoken` 6 _dialogue_widget_ref_10))
    (:`12`
      ; Ghost Times Spoken: 12
      (set `/Game/Dialogue/WBP_Dialogue.Ghost_Text` "I am The Ghost of the Archive, I don’t have any name, I am just here to help." _dialogue_widget_ref_14)
      (`Widget.SetVisibility` (`/Game/Dialogue/WBP_Dialogue.Continue_Button` _dialogue_widget_ref_14) "Visible")
      (`Widget.SetVisibility` (`/Game/Dialogue/WBP_Dialogue.Player_Dialogue_Box` _dialogue_widget_ref_14) "Hidden"))
    (:`13`
      ; Ghost Times Spoken: 13
      (`Widget.SetVisibility` (`/Game/Dialogue/WBP_Dialogue.Player_Dialogue_Box` _dialogue_widget_ref_2) "Visible")
      (`Widget.SetVisibility` (`/Game/Dialogue/WBP_Dialogue.Continue_Button` _dialogue_widget_ref_2) "Hidden")
      (set `/Game/Dialogue/WBP_Dialogue.Ghost_Text` "Need something?" _dialogue_widget_ref_2)
      (set `/Game/Dialogue/WBP_Dialogue.Option1_Text` "I need help..." _dialogue_widget_ref_2)
      (set `/Game/Dialogue/WBP_Dialogue.Option2_Text` "Who are you?" _dialogue_widget_ref_2)
      (set `/Game/Dialogue/WBP_Dialogue.Option3_Text` "About the archive..." _dialogue_widget_ref_2)
      (`Widget.SetIsEnabled` (`/Game/Dialogue/WBP_Dialogue.Option_3_Button` (`self.Dialogue_Widget_REF`)) true)
      (set `/Game/Dialogue/WBP_Dialogue.Option4_Text` "I'm good" _dialogue_widget_ref_2)
      (`Widget.SetIsEnabled` (`/Game/Dialogue/WBP_Dialogue.Option_4_Button` (`self.Dialogue_Widget_REF`)) true))
    (:`14`
      ; Ghost Times Spoken: 14
      (set `/Game/Dialogue/WBP_Dialogue.Ghost_Text` "You can interact with anything that has an outline. You can even grab a soda, but remember to throw the box in the trash after." _dialogue_widget_ref_15)
      (`Widget.SetVisibility` (`/Game/Dialogue/WBP_Dialogue.Continue_Button` _dialogue_widget_ref_15) "Visible")
      (`Widget.SetVisibility` (`/Game/Dialogue/WBP_Dialogue.Player_Dialogue_Box` _dialogue_widget_ref_15) "Hidden"))
    (:`15`
      ; Ghost Times Spoken: 15
      (set `/Game/Dialogue/WBP_Dialogue.Ghost_Text` "There are paintings to read about and posters to learn from. Make sure to look for info posters, as they give away essential information." _dialogue_widget_ref_16)
      (`Widget.SetVisibility` (`/Game/Dialogue/WBP_Dialogue.Continue_Button` _dialogue_widget_ref_16) "Visible")
      (`Widget.SetVisibility` (`/Game/Dialogue/WBP_Dialogue.Player_Dialogue_Box` _dialogue_widget_ref_16) "Hidden")
      (set `/Game/Dialogue/WBP_Dialogue.Ghost_Times_Spoken` 6 _dialogue_widget_ref_16))
    (:`16`
      ; Ghost Times Spoken: 16 (Close Widget)
      (`/Game/Dialogue/WBP_Dialogue.Close Dialogue` (`self.Dialogue_Widget_REF`))
      (set `self.Is_Dialogue_Open?` false))))

(event `/Game/Blueprint/Lock_System/BPI_Interact.Interact`
  ; When Interacted with add the dialogue widget to the viewport, hide the interact widget, and choose dialogue based on Ghost Times Spoken number
  (`UserWidget.AddToViewport` (`self.Dialogue_Widget_REF`) 0)
  (set `self.Is_Dialogue_Open?` true)
  (`self.Hide Interact`)
  (goto _label_3))

(fn `Get Name`
  (returns (Name :type Text))
  (return ""))

(fn `UserConstructionScript`)