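; MinigamePopUp_Shredded is a trigger actor that shows a pop-up widget, apparently for the Shredded minigame, while something overlaps its box.
; On begin overlap it creates a new PopUp5, assigns it to the widget component, makes that visible and plays PopUpAnimation.
; On end overlap it clears the stored widget reference and hides the component.
; Neither event filters the overlapping actor.
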(event `self.Box.OnComponentBeginOverlap`
  (params (OverlappedComponent :type "PrimitiveComponent Object Reference") (OtherActor :type "Actor Object Reference") (OtherComp :type "PrimitiveComponent Object Reference") (OtherBodyIndex :type Integer) (bFromSweep :type Boolean) (SweepResult :type "HitResult Structure (by ref)"))
  (bind _widget (`self.Widget`))
  ; CollisionBox PopUp & Outline
  (bind _returnvalue (`|CreateWidget` "/Game/Blueprint/PopUp_Widgets/PopUp5.PopUp5_C"))
  (bind _output_get (set `self.NewVar_0` _returnvalue))
  (`WidgetComponent.SetWidget` _widget _output_get)
  (`SceneComponent.SetVisibility` _widget true false)
  (bind _newvar_0 (`self.NewVar_0`)
    (:`then`
      (`UserWidget.PlayAnimation` _newvar_0 (`/Game/Blueprint/PopUp_Widgets/PopUp5.PopUpAnimation` _newvar_0) 0.0 1 "Forward" 1.0 false))
    (:`else`)))

(event `self.Box.OnComponentEndOverlap`
  (params (OverlappedComponent :type "PrimitiveComponent Object Reference") (OtherActor :type "Actor Object Reference") (OtherComp :type "PrimitiveComponent Object Reference") (OtherBodyIndex :type Integer))
  ; CollisionBox PopUp & Outline
  (set `self.NewVar_0` null)
  (`SceneComponent.SetVisibility` (`self.Widget`) false false))

(fn `UserConstructionScript`)