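; BP_Vending_Machine is an interactable vending machine that dispenses a random soda actor.
; An overlap box toggles the interact prompt widget for BP_Archivist.
; The OneSodaPlease event spawns one of three soda classes just in front of ExitPoint and plays a sound.
; A DoOnce paired with a delay enforces a cooldown between dispenses, showing the Button countdown component until it resets.
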(event `self.Widget Visibility Box.OnComponentBeginOverlap`
  (params (OverlappedComponent :type "PrimitiveComponent Object Reference") (OtherActor :type "Actor Object Reference") (OtherComp :type "PrimitiveComponent Object Reference") (OtherBodyIndex :type Integer) (bFromSweep :type Boolean) (SweepResult :type "HitResult Structure (by ref)"))
  ; Shows e to interact widget when in collision box
  (cast `/Game/Blueprint/BP_Archivist` OtherActor)
  (`SceneComponent.SetHiddenInGame` (`self.Widget`) false false))

(event `self.Widget Visibility Box.OnComponentEndOverlap`
  (params (OverlappedComponent :type "PrimitiveComponent Object Reference") (OtherActor :type "Actor Object Reference") (OtherComp :type "PrimitiveComponent Object Reference") (OtherBodyIndex :type Integer))
  ; Shows e to interact widget when in collision box
  (cast `/Game/Blueprint/BP_Archivist` OtherActor)
  (`SceneComponent.SetHiddenInGame` (`self.Widget`) true false))

(event `/Game/Blueprint/Quest_System/I_Interaction_Interface.One Soda Please`
  (bind _exit_point (`self.Exit Point`))
  ; Spawns soda can
  (`/Engine/EditorBlueprintResources/StandardMacros.DoOnce` false :!label _label
    (:`Completed`
      (`|SpawnActorFromClass` (select `int` (`KismetMathLibrary.RandomIntegerInRange` 0 2) :`0` (`self.Soda Can`) :`1` (`self.Soda`) :`2` (`self.Soda Box`)) (`KismetMathLibrary.MakeTransform` (+ (`SceneComponent.K2_GetComponentLocation` _exit_point) (`SceneComponent.GetForwardVector` _exit_point))) "Undefined" "MultiplyWithRoot" null null)
      ; Plays sound
      (`GameplayStatics.PlaySound2D` "/Game/Sounds/SFX/SFX_Vending_Machine.SFX_Vending_Machine" 1.0 1.0 0.0 null null)
      ; Delays and sets hidden of countdown
      (`SceneComponent.SetHiddenInGame` (`self.button`) false false)
      (`KismetSystemLibrary.Delay` 10.0)
      (`SceneComponent.SetHiddenInGame` (`self.button`) true false)
      (goto _label :!via `Reset`))))

(fn `UserConstructionScript`)