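; BP_Trash is a trash actor in the vending machine folder that disposes of sodas when its collision box is overlapped.
; Any overlap randomly picks SodaCan, Soda or SodaBox and destroys every actor of that class in the level, regardless of what entered the box.
; Each destruction plays a 2D sound and hides the Niagara effect, which a short Delay inside the loop makes visible again.
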(event `self.Box.OnComponentBeginOverlap`
  (params (OverlappedComponent :type "PrimitiveComponent Object Reference") (OtherActor :type "Actor Object Reference") (OtherComp :type "PrimitiveComponent Object Reference") (OtherBodyIndex :type Integer) (bFromSweep :type Boolean) (SweepResult :type "HitResult Structure (by ref)"))
  ; Destroys soda on impact with collision box
  (bind _outactors (`GameplayStatics.GetAllActorsOfClass` (select `int` (`KismetMathLibrary.RandomIntegerInRange` 0 2) :`0` (`self.Soda Can`) :`1` (`self.Soda`) :`2` (`self.Soda Box`) :`3` null :!type "Actor Class Reference")))
  (for _array_element _outactors
    (`self.K2_DestroyActor` _array_element)
    ; Plays sound, Shows and hides niagara after 0.5 seconds
    (`GameplayStatics.PlaySound2D` "/Engine/VREditor/Sounds/UI/Foliage_Placed.Foliage_Placed" 1.0 1.0 0.0 null null)
    (`SceneComponent.SetHiddenInGame` (`self.Niagara`) true false)
    (`KismetSystemLibrary.Delay` 0.5)
    (`SceneComponent.SetHiddenInGame` (`self.Niagara`) false false)))

(fn `UserConstructionScript`)