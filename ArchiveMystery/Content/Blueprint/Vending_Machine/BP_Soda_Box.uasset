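; BP_Soda_Box is a vending machine soda item that plays drop sounds when it hits objects or the floor.
; On Hit, a DoOnce gate plays one of two random can-drop sounds at the impact point, then resets after a short delay.
; Volume scales with the Soda component's X velocity alone, clamped to a maximum.
; A GetName function exposes the item's Name.
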(event `self.ReceiveHit`
  (params (MyComp :type "PrimitiveComponent Object Reference") (Other :type "Actor Object Reference") (OtherComp :type "PrimitiveComponent Object Reference") (bSelfMoved :type Boolean) (HitLocation :type "Vector Structure") (HitNormal :type "Vector Structure") (NormalImpulse :type "Vector Structure") (Hit :type "HitResult Structure (by ref)"))
  (bind _returnvalue (`KismetMathLibrary.FClamp` (/ (`KismetMathLibrary.VSize` (`KismetMathLibrary.Conv_DoubleToVector` (.x (`SceneComponent.GetComponentVelocity` (`self.Soda`))))) 1200.0) 0.0 0.7))
  ; Create sound when hit against objects and floor
  (`/Engine/EditorBlueprintResources/StandardMacros.DoOnce` false :!label _label
    (:`Completed`
      (switch `int` (`KismetMathLibrary.RandomInteger` 2)
        (:`0`
          (`GameplayStatics.SpawnSoundAtLocation` "/Game/Sounds/SFX/SFX_Soda_Can_Drop_1.SFX_Soda_Can_Drop_1" HitLocation (struct) _returnvalue 1.0 0.0 null null))
        (:`1`
          (`GameplayStatics.SpawnSoundAtLocation` "/Game/Sounds/SFX/SFX_Soda_Can_Drop_2.SFX_Soda_Can_Drop_2" HitLocation (struct) _returnvalue 1.0 0.0 null null)))
      (`KismetSystemLibrary.Delay` 0.2)
      (goto _label :!via `Reset`))))

(fn `Get Name`
  (returns (Name :type Text))
  (return (`self.Name`)))

(fn `UserConstructionScript`)