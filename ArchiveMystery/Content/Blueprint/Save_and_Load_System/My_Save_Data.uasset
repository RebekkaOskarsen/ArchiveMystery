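; My_Save_Data is a save data Blueprint that stores and restores the player's quest state.
; SaveQuestLog copies the active and completed quest lists from a quest log, while SaveQuestDetails records each quest's stage and objective progress in a map keyed by quest ID.
; LoadQuests re-adds active quests to the log, applies any saved stage and progress, then restores both lists.
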(fn `Load Quests`
  (params (`Quest Log` :type "/Game/Blueprint/Quest_System/BAC_Quest_Log Object Reference"))
  (for _array_element (`self.CurrentActiveQuests`)
    (bind _quest (`/Game/Blueprint/Quest_System/BAC_Quest_Log.Add New Quest` `Quest Log` _array_element))
    (bind (_value _returnvalue) (`BlueprintMapLibrary.Map_Find` (`self.QuestProgress`) _array_element))
    (if _returnvalue
      (bind (_progress _currentstage) (break `/Game/Blueprint/Save_and_Load_System/S_QuestSaveData` _value))
      (set `/Game/Blueprint/Quest_System/BP_Quest_Base.Current Stage` _currentstage _quest)
      (set `/Game/Blueprint/Quest_System/BP_Quest_Base.Current Objective Progress` _progress _quest)))
  (set `/Game/Blueprint/Quest_System/BAC_Quest_Log.Current Active Quests` (`self.CurrentActiveQuests`) `Quest Log`)
  (set `/Game/Blueprint/Quest_System/BAC_Quest_Log.Completed Quests` (`self.CompletedQuests`) `Quest Log`))

(fn `Save Quest Details`
  (params (Quest :type "/Game/Blueprint/Quest_System/BP_Quest_Base Object Reference"))
  (returns (QuestProgress :type "Map of Name to /Game/Blueprint/Save_and_Load_System/S_QuestSaveData Structure"))
  (bind _questprogress (`self.QuestProgress`))
  (`BlueprintMapLibrary.Map_Add` _questprogress (`/Game/Blueprint/Quest_System/BP_Quest_Base.QuestID` Quest) (make `/Game/Blueprint/Save_and_Load_System/S_QuestSaveData` (`/Game/Blueprint/Quest_System/BP_Quest_Base.Current Objective Progress` Quest) (`/Game/Blueprint/Quest_System/BP_Quest_Base.Current Stage` Quest)))
  (return _questprogress))

(fn `SaveQuestLog`
  (params (`Quest Log` :type "/Game/Blueprint/Quest_System/BAC_Quest_Log Object Reference"))
  (set `self.CurrentActiveQuests` (`/Game/Blueprint/Quest_System/BAC_Quest_Log.Current Active Quests` `Quest Log`))
  (set `self.CompletedQuests` (`/Game/Blueprint/Quest_System/BAC_Quest_Log.Completed Quests` `Quest Log`)))