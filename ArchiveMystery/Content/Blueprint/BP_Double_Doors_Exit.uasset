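; BP_Double_Doors_Exit is a double-door exit that brings up the exit-game screen when interacted with.
; Front and back trigger boxes each set an inside flag for BP_Archivist and show or remove a long "E to interact" prompt.
; InteractWith disables character input, switches to UI-only mode with a visible cursor, opens W_Exit_Game and returns "GoHome".
; The inside flags are only written in this Blueprint, never read.
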(event `self.Open Door Collission Front.OnComponentBeginOverlap`
  (params (OverlappedComponent :type "PrimitiveComponent Object Reference") (OtherActor :type "Actor Object Reference") (OtherComp :type "PrimitiveComponent Object Reference") (OtherBodyIndex :type Integer) (bFromSweep :type Boolean) (SweepResult :type "HitResult Structure (by ref)"))
  ; Open Collission
  (cast `/Game/Blueprint/BP_Archivist` OtherActor)
  (set `self.Player Is Inside Front Box` true)
  (bind _returnvalue (`|CreateWidget` "/Game/Blueprint/W_E_To_Interact_Long.W_E_To_Interact_Long_C"))
  (`UserWidget.AddToViewport` _returnvalue 0))

(event `self.Open Door Collission Front.OnComponentEndOverlap`
  (params (OverlappedComponent :type "PrimitiveComponent Object Reference") (OtherActor :type "Actor Object Reference") (OtherComp :type "PrimitiveComponent Object Reference") (OtherBodyIndex :type Integer))
  ; Open Collission
  (cast `/Game/Blueprint/BP_Archivist` OtherActor)
  (set `self.Player Is Inside Front Box` false)
  (`Widget.RemoveFromParent` (stale `self.Open Door Collission Front.OnComponentBeginOverlap` _returnvalue)))

(event `self.Open Door Collission Back.OnComponentBeginOverlap`
  (params (OverlappedComponent :type "PrimitiveComponent Object Reference") (OtherActor :type "Actor Object Reference") (OtherComp :type "PrimitiveComponent Object Reference") (OtherBodyIndex :type Integer) (bFromSweep :type Boolean) (SweepResult :type "HitResult Structure (by ref)"))
  ; Open Collission
  (cast `/Game/Blueprint/BP_Archivist` OtherActor)
  (set `self.Player Is Inside Back Box` true)
  (bind _returnvalue (`|CreateWidget` "/Game/Blueprint/W_E_To_Interact_Long.W_E_To_Interact_Long_C"))
  (`UserWidget.AddToViewport` _returnvalue 0))

(event `self.Open Door Collission Back.OnComponentEndOverlap`
  (params (OverlappedComponent :type "PrimitiveComponent Object Reference") (OtherActor :type "Actor Object Reference") (OtherComp :type "PrimitiveComponent Object Reference") (OtherBodyIndex :type Integer))
  ; Open Collission
  (cast `/Game/Blueprint/BP_Archivist` OtherActor)
  (set `self.Player Is Inside Back Box` false)
  (`Widget.RemoveFromParent` (stale `self.Open Door Collission Back.OnComponentBeginOverlap` _returnvalue)))

(fn `Interact With`
  (returns (ObjectiveID :type String))
  (bind _returnvalue (`GameplayStatics.GetPlayerController` 0))
  (`/Engine/EditorBlueprintResources/StandardMacros.IsValid` _returnvalue
    (:`Is Valid`
      (`self.DisableInput` (`GameplayStatics.GetPlayerCharacter` 0) _returnvalue)
      (`WidgetBlueprintLibrary.SetInputMode_UIOnlyEx` _returnvalue null)
      (set `PlayerController.bShowMouseCursor` true _returnvalue)
      (bind _returnvalue_2 (`|CreateWidget` "/Game/Blueprint/W_Exit_Game.W_Exit_Game_C"))
      (`UserWidget.AddToViewport` _returnvalue_2 0)
      (return "GoHome"))))

(fn `UserConstructionScript`)