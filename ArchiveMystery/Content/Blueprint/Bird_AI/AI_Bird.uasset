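; AI controller for a bird that makes it wander on the ground at random.
; From BeginPlay, it loops AIMoveTo toward a random reachable point offset along the pawn's forward or right axis, pausing briefly after success or failure.
; The walk only starts a move if the pawn's IsFlying interface message returns false.
; A self-repeating RandomFlying event is marked not working and is not triggered from BeginPlay.
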(event `self.ReceiveBeginPlay`
  (`self.Random Walk`))

(event `Random Flying`
  (params (Target :type "Vector Structure"))
  ; Random flying, not working
  (message `/Game/Blueprint/Bird_AI/BPI_Bird_Fly.Fly` (`self.K2_GetPawn`) Target)
  (`KismetSystemLibrary.Delay` (`KismetMathLibrary.RandomFloatInRange` 3.0 5.0))
  (`self.Random Flying` (0.0 0.0 0.0)))

(event `Random Walk`
  (bind _returnvalue (`self.K2_GetPawn`))
  (bind _returnvalue_2 (`KismetMathLibrary.RandomBool`))
  ; Random Walk
  (bind _flying (message `/Game/Blueprint/Bird_AI/BPI_Bird_Fly.IsFlying` _returnvalue :!label _label))
  (if (not _flying)
    (`|AIMoveTo` _returnvalue (`NavigationSystemV1.K2_GetRandomReachablePointInRadius` (+ (`self.K2_GetActorLocation` _returnvalue) (* (`KismetMathLibrary.SelectVector` (`self.GetActorForwardVector` _returnvalue) (`self.GetActorRightVector` _returnvalue) _returnvalue_2) (* (`KismetMathLibrary.RandomFloatInRange` 50.0 100.0) (`KismetMathLibrary.SelectFloat` 1.0 -1.0 _returnvalue_2)))) 200.0 null null) null
      (:`OnSuccess`
        _)
      (:`OnFail`
        _))
    (`KismetSystemLibrary.Delay` (`KismetMathLibrary.RandomFloatInRange` 2.0 4.0))
    (goto _label)))

(fn `UserConstructionScript`)