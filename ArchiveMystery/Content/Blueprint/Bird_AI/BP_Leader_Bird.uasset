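; Flock leader bird character that spawns child birds, wanders on foot via AI MoveTo and flees approaching threats.
; Tick steers flight by movement input: birds with a leader hold indexed offsets behind its location updates, others chase a target point.
; Threats sensed by followers go to the leader, which launches the flock and, after a retriggerable delay, lands where the threat was.
; Leaders sensing threats themselves only start their own flight.
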(event `self.ReceiveBeginPlay`
  ; Begin play
  (`KismetSystemLibrary.Delay` 0.2)
  (`self.Spawn Flock`)
  (`KismetSystemLibrary.Delay` 1.0)
  (`self.Random Walk`)
  (set `self.Random Offset` (`KismetMathLibrary.RandomFloatInRange` 50.0 200.0) :!label _label)
  (`KismetSystemLibrary.Delay` 0.2)
  (goto _label))

(event `self.ReceiveTick`
  (params (DeltaSeconds :type "Float (single-precision)"))
  (bind _returnvalue (`self.K2_GetActorLocation`))
  (bind _returnvalue_2 (`self.K2_GetActorLocation`))
  (bind _returnvalue_3 (`self.K2_GetActorLocation`))
  (bind _land_location (`self.Land Location`))
  (bind _flight_target_location (`self.Flight Target Location`))
  (bind _returnvalue_4 (+ (`self.K2_GetActorLocation` (`self.Leader Bird`)) (`KismetMathLibrary.MakeVector` (* (`self.Flock Index`) (`self.Random Offset`)) 0.0 -50.0)))
  ; The birds can take-off (Flying Movement)
  (switch `EMovementMode` (`CharacterMovementComponent.MovementMode` (`self.CharacterMovement`))
    (:`MOVE_Flying`
      (if (`self.Land`)
        ;; Landing
        (if (> (`KismetMathLibrary.Vector_Distance` _returnvalue_2 _land_location) 50.0)
          (`self.AddMovementInput` (`KismetMathLibrary.GetDirectionUnitVector` _returnvalue_2 _land_location))
          (else
            (`self.Land On Ground` self)
            (`self.Land On Ground` (`self.Flock`))))
        (else
          (`/Engine/EditorBlueprintResources/StandardMacros.IsValid` (`self.Leader Bird`)
            (:`Is Valid`
              ;; Follower Flying
              (if (> (`KismetMathLibrary.Vector_Distance` _returnvalue _returnvalue_4) 100.0)
                (`self.AddMovementInput` (`KismetMathLibrary.GetDirectionUnitVector` _returnvalue _returnvalue_4) 1.0 true)))
            (:`Is Not Valid`
              ;; Random Flying
              (if (< (`KismetMathLibrary.VSize` (- _flight_target_location _returnvalue_3)) 200.0)
                (set `self.Flight Target Location` (+ _flight_target_location (5000.0 5000.0 100.0))))
              (`self.AddMovementInput` (`KismetMathLibrary.GetDirectionUnitVector` _returnvalue_3 _flight_target_location) 1.0 true))))))))

(event `self.Fly`
  (params (`Target Location` :type "Vector Structure"))
  ; The birds fly
  (set `self.Flight Target Location` `Target Location`)
  (`KismetSystemLibrary.Delay` (`KismetMathLibrary.RandomFloatInRange` 0.1 0.9))
  (`CharacterMovementComponent.SetMovementMode` (`self.CharacterMovement`) "MOVE_Flying" 0)
  (`MovementComponent.StopMovementImmediately` (`self.CharacterMovement`)))

(event `self.Threat Collision.OnComponentBeginOverlap`
  (params (OverlappedComponent :type "PrimitiveComponent Object Reference") (OtherActor :type "Actor Object Reference") (OtherComp :type "PrimitiveComponent Object Reference") (OtherBodyIndex :type Integer) (bFromSweep :type Boolean) (SweepResult :type "HitResult Structure (by ref)"))
  (bind _leader_bird (`self.Leader Bird`))
  ; Alerting
  (bind _threat (message `/Game/Blueprint/Bird_AI/BPI_NPC_Character.Is Threat` OtherActor))
  (if _threat
    (`/Engine/EditorBlueprintResources/StandardMacros.IsValid` _leader_bird
      (:`Is Valid`
        (`self.Report Threat` _leader_bird OtherActor))
      (:`Is Not Valid`
        (`self.Start Flying` OtherActor)))))

(event `Spawn Flock`
  ; Spawn flock from leader bird
  (if (> (`self.Flock_Size`) 0)
    (for _index (range (+ (`self.Flock_Size`) 1))
      (bind _returnvalue (`|SpawnActorFromClass` "/Game/Blueprint/Bird_AI/BP_Child_Bird.BP_Child_Bird_C" (`KismetMathLibrary.MakeTransform` (`NavigationSystemV1.K2_GetRandomReachablePointInRadius` (`self.K2_GetActorLocation`) 500.0 null null) (`KismetMathLibrary.MakeRotator` 0.0 0.0 (`KismetMathLibrary.RandomFloatInRange` 0.0 360.0)) (* (1.0 1.0 1.0) (`KismetMathLibrary.RandomFloatInRange` 0.8 1.0))) "AdjustIfPossibleButDontSpawnIfColliding" "MultiplyWithRoot" null null))
      (`/Engine/EditorBlueprintResources/StandardMacros.IsValid` _returnvalue
        (:`Is Valid`
          (`KismetArrayLibrary.Array_Add` (`self.Flock`) _returnvalue)
          (set `/Game/Blueprint/Bird_AI/BP_Leader_Bird.Leader Bird` self _returnvalue)
          (set `/Game/Blueprint/Bird_AI/BP_Leader_Bird.Flock Index` _index _returnvalue))))
    (for _array_element (`self.Flock`)
      (`self.SpawnDefaultController` _array_element))))

(event `Random Flying`
  (params (Target :type "Vector Structure"))
  ; Random flying
  (`/Game/Blueprint/Bird_AI/BPI_Bird_Fly.Fly` self Target)
  (`KismetSystemLibrary.Delay` (`KismetMathLibrary.RandomFloatInRange` 3.0 5.0))
  (bind _flying (`self.IsFlying`))
  (if _flying
    (`self.Random Flying` self (+ (`KismetMathLibrary.RandomPointInBoundingBox` (+ (`self.K2_GetActorLocation` self) (* (`KismetMathLibrary.SelectVector` (`self.GetActorForwardVector` self) (`self.GetActorRightVector` self) (`KismetMathLibrary.RandomBool`)) (`KismetMathLibrary.RandomFloatInRange` 50000.0 80000.0))) (1000.0 1000.0 1000.0)) (0.0 0.0 30000.0)))))

(event `Random Walk`
  (bind _returnvalue (`KismetMathLibrary.RandomBool`))
  ; Random Walk
  (bind _flying (`/Game/Blueprint/Bird_AI/BPI_Bird_Fly.IsFlying` self :!label _label_2))
  (if (not _flying)
    (switch `EMovementMode` (`CharacterMovementComponent.MovementMode` (`self.CharacterMovement`))
      (:`MOVE_Walking`
        (`|AIMoveTo` self (`NavigationSystemV1.K2_GetRandomReachablePointInRadius` (+ (`self.K2_GetActorLocation` self) (* (`KismetMathLibrary.SelectVector` (`self.GetActorForwardVector` self) (`self.GetActorRightVector` self) _returnvalue) (* (`KismetMathLibrary.RandomFloatInRange` 50.0 100.0) (`KismetMathLibrary.SelectFloat` 1.0 -1.0 _returnvalue)))) 200.0 null null) null
          (:`OnSuccess`
            _)
          (:`OnFail`
            _))
        (`KismetSystemLibrary.Delay` (`KismetMathLibrary.RandomFloatInRange` 2.0 4.0))
        (goto _label_2)))))

(event `Report Threat`
  (params (Threat :type "Actor Object Reference"))
  ; When player approaches, all birds in the same flock flies away together.
  (`self.Start Flying` Threat)
  (`KismetSystemLibrary.Delay` 0.3)
  (for _array_element (`self.Flock`)
    (`self.Fly` _array_element (+ (`self.K2_GetActorLocation`) (0.0 0.0 1000.0))))
  ;; How long it takes for the birds to come flying back.
  (`KismetSystemLibrary.RetriggerableDelay` 10.0)
  (set `self.Land` true))

(event `Land On Ground`
  (bind _flock (`self.Flock`))
  ; Landing on ground (Leader)
  (`CharacterMovementComponent.SetMovementMode` (`self.CharacterMovement`) "MOVE_Walking" 0)
  (set `self.Land` false)
  (`KismetSystemLibrary.Delay` (`KismetMathLibrary.RandomFloatInRange` 1.0 2.0))
  (`self.Random Walk`)
  (`self.Random Walk` _flock)
  (for _array_element _flock
    (set `self.Land Location` (`NavigationSystemV1.K2_GetRandomReachablePointInRadius` (`self.K2_GetActorLocation`) 1000.0 null null))
    (set `/Game/Blueprint/Bird_AI/BP_Leader_Bird.Land` true _array_element)))

(fn `IsFlying`
  (returns (Flying :type Boolean))
  (return false))

(fn `UserConstructionScript`)