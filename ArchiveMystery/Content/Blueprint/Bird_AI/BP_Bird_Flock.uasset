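; BP_Bird_Flock is a bird flock actor that flies along the spline of a BP_Path_Birds actor.
; Every Tick it finds that path actor by class and calls StartMoving, which plays a Timeline.
; The Timeline's Alpha maps to a distance along the spline, setting the flock's world location and rotation on each update.
; Timeline length determines flight speed.
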(event `self.ReceiveTick`
  (params (DeltaSeconds :type "Float (single-precision)"))
  (bind _returnvalue (`GameplayStatics.GetActorOfClass` "/Game/Blueprint/Bird_AI/BP_Path_Birds.BP_Path_Birds_C"))
  (set `self.Bird path` _returnvalue)
  (`self.Start Moving`))

(event `Start Moving`
  ; Adjust timeline length for speed
  (bind (_direction _alpha) (`Timeline|Timeline`)
    (:`Update`
      (bind (_returnvalue_location _returnvalue_rotation) (`KismetMathLibrary.BreakTransform` (`SplineComponent.GetTransformAtDistanceAlongSpline` (`/Game/Blueprint/Bird_AI/BP_Path_Birds.Spline` (`self.Bird path`)) (`KismetMathLibrary.Lerp` 0.0 (`SplineComponent.GetSplineLength` (`/Game/Blueprint/Bird_AI/BP_Path_Birds.Spline` (`self.Bird path`))) _alpha) "World" false)))
      (`self.K2_SetActorLocationAndRotation` _returnvalue_location _returnvalue_rotation))))

(fn `UserConstructionScript`)