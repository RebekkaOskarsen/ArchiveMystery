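; Bird character that takes flight when the BP_Archivist enters its threat collision.
; The overlap calls Fly with the stored flight target, which switches CharacterMovement to Flying mode.
; While flying, Tick adds forced movement input toward that target and shifts it by a fixed horizontal offset whenever the bird gets close, so it keeps flying onward.
; IsFlying reports whether that movement mode is active.
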(event `self.ReceiveTick`
  (params (DeltaSeconds :type "Float (single-precision)"))
  (bind _flight_target_location (`self.Flight Target Location`))
  (bind _returnvalue (- _flight_target_location (`self.K2_GetActorLocation`)))
  ; The birds can take-off
  (switch `EMovementMode` (`CharacterMovementComponent.MovementMode` (`self.CharacterMovement`))
    (:`MOVE_Flying`
      (if (< (`KismetMathLibrary.VSize` _returnvalue) 200.0)
        (set `self.Flight Target Location` (+ _flight_target_location (5000.0 5000.0 0.0))))
      (`self.AddMovementInput` (`KismetMathLibrary.Normal` _returnvalue) 1.0 true))))

(event `/Game/Blueprint/Bird_AI/BPI_Bird_Fly.Fly`
  (params (`Target Location` :type "Vector Structure"))
  ; The birds fly
  (set `self.Flight Target Location` `Target Location`)
  (`CharacterMovementComponent.SetMovementMode` (`self.CharacterMovement`) "MOVE_Flying" 0))

(event `self.Threat Collision.OnComponentBeginOverlap`
  (params (OverlappedComponent :type "PrimitiveComponent Object Reference") (OtherActor :type "Actor Object Reference") (OtherComp :type "PrimitiveComponent Object Reference") (OtherBodyIndex :type Integer) (bFromSweep :type Boolean) (SweepResult :type "HitResult Structure (by ref)"))
  ; Birds fly once character overlaps collision
  (cast `/Game/Blueprint/BP_Archivist` OtherActor)
  (`self.Fly` (`self.Flight Target Location`)))

(fn `IsFlying`
  (returns (Flying :type Boolean))
  (return (`|EnumEquality` (`CharacterMovementComponent.MovementMode` (`self.CharacterMovement`)) "MOVE_Flying")))

(fn `UserConstructionScript`)