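; A movable archive shelf that the player slides right and left with buttons.
; Overlapping the collision box as BP_Archivist shows the interact prompt and dot widgets, removed on exit.
; LookatRight and LookatLeft play a button sound and drive one timeline forward or in reverse to move the shelf.
; Paired DoOnce gates and a direction flag alternate the two moves, and a separate event can stop the timeline.
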(event `self.Collision Box.OnComponentBeginOverlap`
  (params (OverlappedComponent :type "PrimitiveComponent Object Reference") (OtherActor :type "Actor Object Reference") (OtherComp :type "PrimitiveComponent Object Reference") (OtherBodyIndex :type Integer) (bFromSweep :type Boolean) (SweepResult :type "HitResult Structure (by ref)"))
  ; Shows widget
  (cast `/Game/Blueprint/BP_Archivist` OtherActor)
  (bind _returnvalue (`|CreateWidget` "/Game/Blueprint/W_E_To_Interact_Long.W_E_To_Interact_Long_C"))
  (bind _output_get (set `self.E Widget` _returnvalue))
  (`UserWidget.AddToViewport` _output_get 0)
  (bind _returnvalue_2 (`|CreateWidget` "/Game/Blueprint/W_Dot.W_Dot_C"))
  (bind _output_get_2 (set `self.Dot` _returnvalue_2))
  (`UserWidget.AddToViewport` _output_get_2 0))

(event `self.Collision Box.OnComponentEndOverlap`
  (params (OverlappedComponent :type "PrimitiveComponent Object Reference") (OtherActor :type "Actor Object Reference") (OtherComp :type "PrimitiveComponent Object Reference") (OtherBodyIndex :type Integer))
  ; Shows widget
  (cast `/Game/Blueprint/BP_Archivist` OtherActor)
  (`Widget.RemoveFromParent` (`self.E Widget`))
  (`Widget.RemoveFromParent` (`self.Dot`)))

(event `Move Shelf Right`
  ; Shelf animation left and right
  (set `self.Shelf has moved right` false)
  (`/Engine/EditorBlueprintResources/StandardMacros.DoOnce` false :!label _label
    (:`Completed`
      (bind (_direction _newtrack_0) (`Timeline|Moves Shelf Right` :!via `PlayFromStart` :!label _label_2)
        (:`Update`
          (`SceneComponent.K2_SetRelativeTransform` (`self.Shelf`) (`KismetMathLibrary.MakeTransform` (* (`KismetMathLibrary.Lerp` _newtrack_0) (`self.New Transform Location`))) false false)
          (if (`self.Shelf has moved right`)
            (goto _label :!via `Reset`)
            (else
              (goto _label_3 :!via `Reset`))))))))

(event `Can't Move Shelf`
  (goto _label_2 :!via `Stop`))

(event `Move Shelf Left`
  ; Shelf animation left and right
  (set `self.Shelf has moved right` true)
  (`/Engine/EditorBlueprintResources/StandardMacros.DoOnce` false :!label _label_3
    (:`Completed`
      (goto _label_2 :!via `Reverse`))))

(event `/Game/Blueprint/Quest_System/I_Interaction_Interface.Look At Right`
  ; Interacted with left and right button, plays animation
  (`/Engine/EditorBlueprintResources/StandardMacros.IsValid` (`GameplayStatics.GetPlayerController` 0)
    (:`Is Valid`
      (`self.Move Shelf Right`)
      (`GameplayStatics.PlaySoundAtLocation` "/Game/Sounds/SFX/SFX_Archive_Button.SFX_Archive_Button" (`self.K2_GetActorLocation`) (struct) 0.5 1.0 0.0 null null null null))))

(event `/Game/Blueprint/Quest_System/I_Interaction_Interface.Look At Left`
  ; Interacted with left and right button, plays animation
  (`/Engine/EditorBlueprintResources/StandardMacros.IsValid` (`GameplayStatics.GetPlayerController` 0)
    (:`Is Valid`
      (`self.Move Shelf Left`)
      (`GameplayStatics.PlaySoundAtLocation` "/Game/Sounds/SFX/SFX_Archive_Button.SFX_Archive_Button" (`self.K2_GetActorLocation`) (struct) 0.5 1.0 0.0 null null null null))))

(fn `Interact With`
  (returns (ObjectiveID :type String)))

(fn `UserConstructionScript`)