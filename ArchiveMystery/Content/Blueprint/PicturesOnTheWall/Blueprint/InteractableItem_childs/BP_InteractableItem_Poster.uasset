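; Interactable wall poster that shows an animated "E" pop-up widget while the Archivist overlaps its box.
; Interact, an interface event, blends the view to the poster's camera, enters cinematic mode with UI-only input, and adds a configurable widget plus website buttons.
; The buttons' exit event blends back to the player, restores game input and removes both widgets.
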(event `self.ReceiveBeginPlay`
  (`self.EnableInput` (`GameplayStatics.GetPlayerController` 0)))

(event `self.Box.OnComponentBeginOverlap`
  (params (OverlappedComponent :type "PrimitiveComponent Object Reference") (OtherActor :type "Actor Object Reference") (OtherComp :type "PrimitiveComponent Object Reference") (OtherBodyIndex :type Integer) (bFromSweep :type Boolean) (SweepResult :type "HitResult Structure (by ref)"))
  (bind _widget (`self.Widget`))
  ; Popup widget with animation
  (cast `/Game/Blueprint/BP_Archivist` OtherActor)
  (bind _returnvalue (`|CreateWidget` "/Game/Blueprint/PopUp_Widgets/WBP_E_PopUp.WBP_E_PopUp_C"))
  (bind _output_get (set `self.InteractionWidget1` _returnvalue))
  (`WidgetComponent.SetWidget` _widget _output_get)
  (`SceneComponent.SetVisibility` _widget true false)
  (bind _interactionwidget1 (`self.InteractionWidget1`)
    (:`then`
      (`UserWidget.PlayAnimation` _interactionwidget1 (`/Game/Blueprint/PopUp_Widgets/WBP_E_PopUp.PopUpAnimation` _interactionwidget1) 0.0 1 "Forward" 1.0 false))
    (:`else`)))

(event `self.Box.OnComponentEndOverlap`
  (params (OverlappedComponent :type "PrimitiveComponent Object Reference") (OtherActor :type "Actor Object Reference") (OtherComp :type "PrimitiveComponent Object Reference") (OtherBodyIndex :type Integer))
  ; Popup widget with animation
  (cast `/Game/Blueprint/BP_Archivist` OtherActor)
  (set `self.InteractionWidget1` null)
  (`SceneComponent.SetVisibility` (`self.Widget`) false false))

(event `self.interact`
  (bind _returnvalue (`GameplayStatics.GetPlayerController` 0))
  ; Interaction, camera and widget
  ;; Interface, referenced in archivist bp
  ;; Move camera, add widget
  (`PlayerController.SetViewTargetWithBlend` _returnvalue (`self.Camera`) 0.3 "VTBlend_Linear" 0.0 false)
  (`PlayerController.SetCinematicMode` _returnvalue true true true true true)
  (`WidgetBlueprintLibrary.SetInputMode_UIOnlyEx` _returnvalue null)
  (set `PlayerController.bShowMouseCursor` true _returnvalue)
  (bind _returnvalue_2 (`|CreateWidget` (`self.Widget_Class`) _returnvalue))
  (`UserWidget.AddToViewport` _returnvalue_2 0)
  (bind _returnvalue_3 (`|CreateWidget` "/Game/Blueprint/PicturesOnTheWall/Blueprint/Widgets/WBP_Website_Buttons.WBP_Website_Buttons_C"))
  (`UserWidget.AddToViewport` _returnvalue_3 0)
  (add `/Game/Blueprint/PicturesOnTheWall/Blueprint/Widgets/WBP_Website_Buttons.OnExitClicked` _returnvalue_3 (delegate `Remove Widget event`)))

(event `Remove Widget event`
  (bind _returnvalue (`GameplayStatics.GetPlayerController` 0))
  ; Interaction, camera and widget
  ;; Revert camera, remove widget
  (`PlayerController.SetViewTargetWithBlend` _returnvalue (`GameplayStatics.GetPlayerCharacter` 0) 0.3 "VTBlend_Linear" 0.0 false)
  (`KismetSystemLibrary.Delay` 0.3)
  (`PlayerController.SetCinematicMode` _returnvalue false true true true true)
  (`WidgetBlueprintLibrary.SetInputMode_GameOnly` _returnvalue)
  (set `PlayerController.bShowMouseCursor` false _returnvalue)
  (`Widget.RemoveFromParent` (stale `self.interact` _returnvalue_2))
  (`Widget.RemoveFromParent` (stale `self.interact` _returnvalue_3))
  (`WidgetBlueprintLibrary.SetFocusToGameViewport`))

(fn `Get Name`
  (returns (Name :type Text))
  (return ""))

(fn `UserConstructionScript`)