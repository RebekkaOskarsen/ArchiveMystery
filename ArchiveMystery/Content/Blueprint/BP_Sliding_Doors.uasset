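; BP_Sliding_Doors is a pair of doors that slide apart when the BP_Archivist enters a trigger box and close when it leaves.
; Overlap begin passes a DoOnce, plays the door sound and runs the Sliding timeline forward; overlap end reverses it without sound.
; Timeline updates lerp both doors' relative X positions in opposite directions and reset the DoOnce on every update.
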(event `self.Box.OnComponentBeginOverlap`
  (params (OverlappedComponent :type "PrimitiveComponent Object Reference") (OtherActor :type "Actor Object Reference") (OtherComp :type "PrimitiveComponent Object Reference") (OtherBodyIndex :type Integer) (bFromSweep :type Boolean) (SweepResult :type "HitResult Structure (by ref)"))
  (cast `/Game/Blueprint/BP_Archivist` OtherActor)
  (`/Engine/EditorBlueprintResources/StandardMacros.DoOnce` false :!label _label
    (:`Completed`
      (`GameplayStatics.PlaySoundAtLocation` "/Game/Sounds/SFX/SFX_Sliding_Doors.SFX_Sliding_Doors" (`self.K2_GetActorLocation`) (struct) 1.0 1.0 0.0 null null null null)
      (bind (_direction _sliding) (`Timeline|Sliding` :!label _label_2)
        (:`Update`
          (`SceneComponent.K2_SetRelativeTransform` (`self.Sliding Door Left`) (`KismetMathLibrary.MakeTransform` (`KismetMathLibrary.MakeVector` (`KismetMathLibrary.Lerp` 123.0 256.0 _sliding))) false false)
          (`SceneComponent.K2_SetRelativeTransform` (`self.Sliding Door Right`) (`KismetMathLibrary.MakeTransform` (`KismetMathLibrary.MakeVector` (`KismetMathLibrary.Lerp` 0.0 -124.0 _sliding))) false false)
          (goto _label :!via `Reset`))))))

(event `self.Box.OnComponentEndOverlap`
  (params (OverlappedComponent :type "PrimitiveComponent Object Reference") (OtherActor :type "Actor Object Reference") (OtherComp :type "PrimitiveComponent Object Reference") (OtherBodyIndex :type Integer))
  (cast `/Game/Blueprint/BP_Archivist` OtherActor)
  (goto _label_2 :!via `Reverse`))

(fn `UserConstructionScript`)