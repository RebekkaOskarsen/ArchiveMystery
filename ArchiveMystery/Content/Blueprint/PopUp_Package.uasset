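; PopUp_Package is an actor that shows an animated pop-up widget when something overlaps its Sphere collision.
; Each begin overlap, with no filter on the overlapping actor, creates a new PopUp4 widget, assigns it to the Widget component, makes it visible and plays PopUpAnimation.
; End overlap does nothing; the reverse-animation and hide logic is present but disconnected, so the pop-up is never hidden here.
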(event `self.Sphere.OnComponentBeginOverlap`
  (params (OverlappedComponent :type "PrimitiveComponent Object Reference") (OtherActor :type "Actor Object Reference") (OtherComp :type "PrimitiveComponent Object Reference") (OtherBodyIndex :type Integer) (bFromSweep :type Boolean) (SweepResult :type "HitResult Structure (by ref)"))
  (bind _widget (`self.Widget`))
  ; CollisionBox PopUp
  (bind _returnvalue (`|CreateWidget` "/Game/Blueprint/PopUp_Widgets/PopUp4.PopUp4_C"))
  (bind _output_get (set `self.InteractionWidget` _returnvalue))
  (`WidgetComponent.SetWidget` _widget _output_get)
  (`SceneComponent.SetVisibility` _widget true false)
  (bind _interactionwidget (`self.InteractionWidget`)
    (:`then`
      (`UserWidget.PlayAnimation` _interactionwidget (`/Game/Blueprint/PopUp_Widgets/PopUp4.PopUpAnimation` _interactionwidget) 0.0 1 "Forward" 1.0 false))
    (:`else`)))

(event `self.Sphere.OnComponentEndOverlap`
  (params (OverlappedComponent :type "PrimitiveComponent Object Reference") (OtherActor :type "Actor Object Reference") (OtherComp :type "PrimitiveComponent Object Reference") (OtherBodyIndex :type Integer))
  ; CollisionBox PopUp
)

(fn `UserConstructionScript`)