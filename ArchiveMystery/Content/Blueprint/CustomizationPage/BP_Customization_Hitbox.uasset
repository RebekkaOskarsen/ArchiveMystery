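; BP_Customization_Hitbox is a trigger actor that opens the customization UI when BP_Archivist enters its Box.
; On overlap begin it disables player character input, switches to UI-only input with the mouse cursor shown, and adds a W_Customization_Button_ widget to the viewport.
; On overlap end with BP_Archivist it destroys itself; this Blueprint never restores input or removes the widget.
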(event `self.Box.OnComponentBeginOverlap`
  (params (OverlappedComponent :type "PrimitiveComponent Object Reference") (OtherActor :type "Actor Object Reference") (OtherComp :type "PrimitiveComponent Object Reference") (OtherBodyIndex :type Integer) (bFromSweep :type Boolean) (SweepResult :type "HitResult Structure (by ref)"))
  (bind _returnvalue (`GameplayStatics.GetPlayerController` 0))
  (cast `/Game/Blueprint/BP_Archivist` OtherActor)
  (`/Engine/EditorBlueprintResources/StandardMacros.IsValid` _returnvalue
    (:`Is Valid`
      (`self.DisableInput` (`GameplayStatics.GetPlayerCharacter` 0) _returnvalue)
      (`WidgetBlueprintLibrary.SetInputMode_UIOnlyEx` _returnvalue null)
      (set `PlayerController.bShowMouseCursor` true _returnvalue)
      (bind _returnvalue_2 (`|CreateWidget` "/Game/Blueprint/CustomizationPage/W_Customization_Button_.W_Customization_Button__C"))
      (bind _output_get (set `self.Widget` _returnvalue_2))
      (`UserWidget.AddToViewport` _output_get 0))))

(event `self.Box.OnComponentEndOverlap`
  (params (OverlappedComponent :type "PrimitiveComponent Object Reference") (OtherActor :type "Actor Object Reference") (OtherComp :type "PrimitiveComponent Object Reference") (OtherBodyIndex :type Integer))
  (cast `/Game/Blueprint/BP_Archivist` OtherActor)
  (`self.K2_DestroyActor`))

(fn `UserConstructionScript`)