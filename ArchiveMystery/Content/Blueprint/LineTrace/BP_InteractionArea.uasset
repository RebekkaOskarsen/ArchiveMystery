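; BP_InteractionArea is an interaction area that relays focus changes to its parent actor.
; ToggleFocus stores the Focused state, forwards it to the parent through an interface message, then shows or hides the component the parent returns as its interaction reference.
; Its own GetInteractionRef is empty, and the nodes for creating and animating an interaction widget are unconnected.
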(event `ToggleFocus`
  (params (Focused :type Boolean))
  (set `self.Focused` Focused)
  (message `/Game/Blueprint/LineTrace/BI_Interaction.Interface_ToggleFocus` (`self.GetParentActor`) (`self.Focused`))
  (bind _ref (message `/Game/Blueprint/LineTrace/BI_Interaction.GetInteractionRef` (`self.GetParentActor`)))
  (`SceneComponent.SetHiddenInGame` _ref (not (`self.Focused`)) false))

(fn `GetInteractionRef`
  (returns (Ref :type "WidgetComponent Object Reference"))
  (return null))

(fn `UserConstructionScript`)