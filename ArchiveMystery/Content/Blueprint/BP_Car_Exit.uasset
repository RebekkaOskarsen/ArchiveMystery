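; Car exit point that lets the player Archivist bring up the exit-game screen.
; Overlapping the front door collision as BP_Archivist sets an inside-box flag and shows an interact prompt widget; leaving clears both.
; The OpensExitWidget event, which has no caller in this Blueprint, adds the exit-game widget to the viewport only while that flag is set.
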(event `self.Open Door Collission Front.OnComponentBeginOverlap`
  (params (OverlappedComponent :type "PrimitiveComponent Object Reference") (OtherActor :type "Actor Object Reference") (OtherComp :type "PrimitiveComponent Object Reference") (OtherBodyIndex :type Integer) (bFromSweep :type Boolean) (SweepResult :type "HitResult Structure (by ref)"))
  ; Open Collission
  (cast `/Game/Blueprint/BP_Archivist` OtherActor)
  (set `self.Player Is Inside Box?` true)
  (bind _returnvalue (`|CreateWidget` "/Game/Blueprint/W_E_To_Interact.W_E_To_Interact_C"))
  (`UserWidget.AddToViewport` _returnvalue 0))

(event `self.Open Door Collission Front.OnComponentEndOverlap`
  (params (OverlappedComponent :type "PrimitiveComponent Object Reference") (OtherActor :type "Actor Object Reference") (OtherComp :type "PrimitiveComponent Object Reference") (OtherBodyIndex :type Integer))
  ; Open Collission
  (cast `/Game/Blueprint/BP_Archivist` OtherActor)
  (set `self.Player Is Inside Box?` false)
  (`Widget.RemoveFromParent` (stale `self.Open Door Collission Front.OnComponentBeginOverlap` _returnvalue)))

(event `Opens Exit Widget`
  ; Opens Exit widget if player is inside box
  (if (`self.Player Is Inside Box?`)
    (bind _returnvalue (`|CreateWidget` "/Game/Blueprint/W_Exit_Game.W_Exit_Game_C"))
    (`UserWidget.AddToViewport` _returnvalue 0)))

(fn `Get Name`
  (returns (Name :type Text))
  (return ""))

(fn `UserConstructionScript`)