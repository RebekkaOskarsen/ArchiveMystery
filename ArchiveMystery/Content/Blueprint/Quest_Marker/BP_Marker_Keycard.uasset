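; Quest marker actor for the keycard objective, showing a W_Quest_Marker through its Widget component.
; On BeginPlay it passes its location to the widget as OriginLocation, the reference for the player-to-marker distance.
; On EndPlay it sets IsMarker3 on ArchiveGameInstance, recording that this marker has left play.
; Its Interact With function is a stub that returns an empty string.
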(event `self.ReceiveBeginPlay`
  ; Calculates distance from player to marker location
  (bind _asw_quest_marker (cast `/Game/Blueprint/Quest_Marker/W_Quest_Marker` (`WidgetComponent.GetWidget` (`self.Widget`))))
  (set `/Game/Blueprint/Quest_Marker/W_Quest_Marker.OriginLocation` (`self.K2_GetActorLocation`) _asw_quest_marker))

(event `self.ReceiveEndPlay`
  (params (EndPlayReason :type "EEndPlayReason Enum" :default "Destroyed"))
  (bind _asarchive_game_instance (cast `ArchiveGameInstance` (`GameplayStatics.GetGameInstance`)))
  (set `ArchiveGameInstance.bIsMarker3` true _asarchive_game_instance))

(fn `Interact With`
  (returns (ObjectiveID :type String))
  (return ""))

(fn `UserConstructionScript`)